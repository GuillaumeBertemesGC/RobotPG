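; Rhythm battle conductor that plays the map's track and drives two robots and directional hit objects from the audio playback time.
; The map is an Alone component loaded in the construction script, and one hidden hit object is spawned per obstacle at BeginPlay.
; Each tick squashes the robots on alternating beats using the map's BPM events.
; Obstacles within the approach window slide from opponent to player, offset by direction.
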(event `AudioProgress`
  (params (PlayingSoundWave :type "SoundWave Object Reference") (PlaybackPercent :type "Float (single-precision)"))
  (set `self.AudioTime` (* PlaybackPercent (`SoundBase.Duration` (`AudioComponent.Sound` (`self.Player`))) 1000.0)))

(event `self.ReceiveBeginPlay`
  (bind _player (`self.Player`))
  (`|ExecutionSequence`
    (:`then_0`
      (add `AudioComponent.OnAudioPlaybackPercent` _player (delegate `AudioProgress`))
      (`AudioComponent.SetSound` _player (`/Game/Scripts/BP/Battle/AC_Map.Track` (`self.Map`)))
      (`AudioComponent.Play` _player 0.0))
    (:`then_1`
      (`self.LoadElements`))))

(event `self.ReceiveTick`
  (params (DeltaSeconds :type "Float (single-precision)"))
  (`|ExecutionSequence`
    (:`then_0`
      (`self.Animate`))
    (:`then_1`
      (`self.PositionElements`))))

(fn `Animate`
  (bind _audiotime (`self.AudioTime`))
  (bind _resultbpm (`self.TakeCurrentBPMEvent`))
  (`|ExecutionSequence`
    (:`then_0`
      (bind _returnvalue (* (/ 60.0 (break `/Game/Scripts/BP/Battle/BPMEvent` _resultbpm)) 1000.0))
      (bind _returnvalue_2 (* _returnvalue 2.0))
      (`self.SetActorScale3D` (`self.RobotSelf`) (`KismetMathLibrary.MakeVector` 1.0 1.0 (`KismetMathLibrary.Lerp` 1.1 1.0 (`|EaseFunction` "EaseOut" (/ (mod (+ (`.Offset_6_B5AD37F142A86B1E2C5E54932E4D08C8` (break `/Game/Scripts/BP/Battle/BPMEvent` _resultbpm)) _audiotime) _returnvalue_2) _returnvalue_2) 0.0 1.0)))))
    (:`then_1`
      (`self.SetActorScale3D` (`self.RobotOponent`) (`KismetMathLibrary.MakeVector` 1.0 1.0 (`KismetMathLibrary.Lerp` 1.1 1.0 (`|EaseFunction` "EaseOut" (/ (mod (+ (+ _audiotime _returnvalue) (`.Offset_6_B5AD37F142A86B1E2C5E54932E4D08C8` (break `/Game/Scripts/BP/Battle/BPMEvent` _resultbpm))) _returnvalue_2) _returnvalue_2) 0.0 1.0)))))))

(fn `LoadElements`
  (`|ExecutionSequence`
    (:`then_0`
      (for _ (`/Game/Scripts/BP/Battle/AC_Map.Obstacles` (`self.Map`))
        (bind _returnvalue (`|SpawnActorFromClass` "/Game/Scripts/BP/Battle/Objs/HitObject.HitObject_C" (`KismetMathLibrary.MakeTransform` (0.0 0.0 0.0) (struct) (0.0 0.0 0.0)) "Undefined" "MultiplyWithRoot" null null))
        (`KismetArrayLibrary.Array_Add` (`self.HitObjects`) _returnvalue)))))

(fn `PositionElements`
  (locals (Offset :type "Vector Structure"))
  (bind _audiotime (`self.AudioTime`))
  (bind _approach_rate (`self.Approach Rate`))
  (for (_array_element _array_index) (`self.HitObjects`)
    (bind (_output_offset _output_direction) (break `/Game/Scripts/BP/Battle/HitObject` (`|GetArrayItem` (`/Game/Scripts/BP/Battle/AC_Map.Obstacles` (`self.Map`)) _array_index)))
    (if (and (> _audiotime (- _output_offset (`self.Approach Rate`))) (< _audiotime _output_offset))
      (`self.SetActorScale3D` _array_element (1.0 1.0 1.0))
      (switch `/Game/Scripts/BP/Battle/Direction` _output_direction
        (:`NewEnumerator0`
          (set `local.Offset` (0.0 0.0 500.0)))
        (:`NewEnumerator1`
          (set `local.Offset` (0.0 0.0 100.0)))
        (:`NewEnumerator2`
          (set `local.Offset` (400.0 0.0 250.0)))
        (:`NewEnumerator3`
          (set `local.Offset` (-400.0 0.0 250.0))))
      (`self.K2_SetActorLocation` _array_element (`KismetMathLibrary.VLerp` (+ (`self.K2_GetActorLocation` (`self.RobotOponent`)) (`local.Offset`)) (+ (* (`local.Offset`) 0.3) (`self.K2_GetActorLocation` (`self.RobotSelf`))) (/ (- (`self.AudioTime`) (- _output_offset _approach_rate)) _approach_rate)) false false)
      (else
        (`self.SetActorScale3D` _array_element (0.0 0.0 0.0))))))

(fn `TakeCurrentBPMEvent`
  (returns (ResultBPM :type "/Game/Scripts/BP/Battle/BPMEvent Structure"))
  (locals (CurrentBPM :type "/Game/Scripts/BP/Battle/BPMEvent Structure"))
  (set `local.CurrentBPM` (make `/Game/Scripts/BP/Battle/BPMEvent` 60.0))
  (for _array_element (`/Game/Scripts/BP/Battle/AC_Map.BPMEvents` (`self.Map`))
    (if (> (`self.AudioTime`) (`.Offset_6_B5AD37F142A86B1E2C5E54932E4D08C8` (break `/Game/Scripts/BP/Battle/BPMEvent` _array_element)))
      (bind _output_get (set `local.CurrentBPM` (make `/Game/Scripts/BP/Battle/BPMEvent` (break `/Game/Scripts/BP/Battle/BPMEvent` _array_element) (`.Offset_6_B5AD37F142A86B1E2C5E54932E4D08C8` (break `/Game/Scripts/BP/Battle/BPMEvent` _array_element))))))
    (return _output_get)))

(fn `UserConstructionScript`
  (bind _returnvalue (`AddComponent|NODE_AddAC_Alone-2`))
  (set `self.Map` _returnvalue)
  (`/Game/Scripts/BP/Battle/Maps/AC_Alone.LoadAlone` _returnvalue))