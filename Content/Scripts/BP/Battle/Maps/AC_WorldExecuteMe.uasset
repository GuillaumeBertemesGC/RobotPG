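; Battle map definition for the song "world.execute(me);" (Mili, Arya Loveday cover), supplying its track, timing and note data.
; LoadMap calls LoadACMap, which sets the track and a single constant-BPM event with an offset, then copies every Opportunities and Obstacles data table row into arrays.
; LoadACMap finishes by calling the parent BeginPlay, while this Blueprint's own BeginPlay and Tick events are disabled.
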(fn `LoadACMap`
  (bind _opportunities_source (`self.Opportunities_Source`))
  (bind _obstacles_source (`self.Obstacles_Source`))
  (`|ExecutionSequence`
    (:`then_0`
      (set `self.Track` "/Game/Scripts/BP/Battle/Tracks/World_execute_me___-_Mili__Arya_Loveday_Cover.World_execute_me___-_Mili__Arya_Loveday_Cover"))
    (:`then_1`
      (set `self.BPMEvents` (`|MakeArray` (make `/Game/Scripts/BP/Battle/BPMEvent` 130.0 1895.0))))
    (:`then_2`
      (bind _outrownames (`DataTableFunctionLibrary.GetDataTableRowNames` _opportunities_source))
      (for _array_element _outrownames
        (bind _returnvalue (`|GetDataTableRow` _opportunities_source _array_element)
          (:`then`
            (`KismetArrayLibrary.Array_Add` (`self.Opportunities`) _returnvalue)))))
    (:`then_3`
      (bind _outrownames_2 (`DataTableFunctionLibrary.GetDataTableRowNames` _obstacles_source))
      (for _array_element_2 _outrownames_2
        (bind _returnvalue_2 (`|GetDataTableRow` _obstacles_source _array_element_2)
          (:`then`
            (`KismetArrayLibrary.Array_Add` (`self.Obstacles`) _returnvalue_2)))))
    (:`then_4`
      (`parent.ReceiveBeginPlay`))))

(fn `LoadMap`
  (`self.LoadACMap`))