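; Battle map component holding the rhythm chart for the track "Alone".
; LoadAlone sets the track, a single BPM event, and lists of timed, directional opportunities and obstacle hit objects, all hard-coded by offset.
; It then calls the parent's BeginPlay, so the inherited setup runs only after the chart is filled, while the component's own BeginPlay does nothing.
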(event `self.ReceiveBeginPlay`)

(fn `LoadAlone`
  (`|ExecutionSequence`
    (:`then_0`
      (set `self.Track` "/Game/Scripts/BP/Battle/Tracks/Alone.Alone"))
    (:`then_1`
      (set `self.BPMEvents` (`|MakeArray` (make `/Game/Scripts/BP/Battle/BPMEvent` 97.3 381.0))))
    (:`then_2`
      (set `self.Opportunities` (`|MakeArray` (make `/Game/Scripts/BP/Battle/Structs/Opportunity` 5315.0) (make `/Game/Scripts/BP/Battle/Structs/Opportunity` 10248.0 "NewEnumerator2") (make `/Game/Scripts/BP/Battle/Structs/Opportunity` 15180.0 "NewEnumerator1") (make `/Game/Scripts/BP/Battle/Structs/Opportunity` 20114.0 "NewEnumerator3") (make `/Game/Scripts/BP/Battle/Structs/Opportunity` 22581.0) (struct))))
    (:`then_3`
      (set `self.Obstacles` (`|MakeArray` (make `/Game/Scripts/BP/Battle/Structs/HitObject` 2848.0) (make `/Game/Scripts/BP/Battle/Structs/HitObject` 7780.0 "NewEnumerator3") (make `/Game/Scripts/BP/Battle/Structs/HitObject` 12714.0 "NewEnumerator1") (make `/Game/Scripts/BP/Battle/Structs/HitObject` 17647.0 "NewEnumerator2") (make `/Game/Scripts/BP/Battle/Structs/HitObject` 21964.0 "NewEnumerator1") (make `/Game/Scripts/BP/Battle/Structs/HitObject` 22889.0 "NewEnumerator1"))))
    (:`then_4`
      (`parent.ReceiveBeginPlay`))))