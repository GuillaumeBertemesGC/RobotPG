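; Music visualiser actor that spawns a row of BP_SoundCubes along X or Y and scales their height to the track's frequency spectrum.
; It assigns the music to BPTrackConductor's player, whose playback-percent callback samples pre-analysed Synesthesia Constant-Q bands to lerp each cube's Z scale.
; Tick derives beat progression from the conductor's current BPM event, gating a subtle bass-driven FOV pulse on GameplayCamera around each beat.
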(event `self.ReceiveBeginPlay`
  (bind _music (`self.Music`))
  (bind _player (`/Game/Scripts/BP/Battle/BP_TrackConductor.Player` (`self.BP_TrackConductor`)))
  (`|ExecutionSequence`
    (:`then_0`
      (`AudioComponent.SetSound` _player _music)
      (set `self.MusicDuration` (`SoundBase.Duration` _music)))
    (:`then_1`
      (bind _soundcubes (`self.SpawnSoundCube` (`self.Nb Sound Cubes`) (`self.Cube Spacing`)))
      (set `self.Sound Cubes` _soundcubes))
    (:`then_2`
      (add `AudioComponent.OnAudioPlaybackPercent` _player (delegate `OnPlayBackChange`)))))

(event `self.ReceiveTick`
  (params (DeltaSeconds :type "Float (single-precision)"))
  (bind _bp_trackconductor (`self.BP_TrackConductor`))
  (bind _resultbpm (`/Game/Scripts/BP/Battle/BP_TrackConductor.TakeCurrentBPMEvent` _bp_trackconductor))
  (bind _returnvalue (* (/ 60.0 (break `/Game/Scripts/BP/Battle/BPMEvent` _resultbpm)) 1000.0))
  (bind _output_get (set `self.AudioBeatProgression` (/ (mod (+ (`.Offset_6_B5AD37F142A86B1E2C5E54932E4D08C8` (break `/Game/Scripts/BP/Battle/BPMEvent` _resultbpm)) (+ (`/Game/Scripts/BP/Battle/BP_TrackConductor.AudioTime` _bp_trackconductor) _returnvalue)) _returnvalue) _returnvalue)))
  (`KismetSystemLibrary.LogString` (`KismetStringLibrary.Conv_DoubleToString` _output_get)))

(event `OnPlayBackChange`
  (params (PlayingSoundWave :type "SoundWave Object Reference") (PlaybackPercent :type "Float (single-precision)"))
  (`self.SynesthesiaScaleSoundCube` (`self.MusicDuration`) PlaybackPercent (`self.Sound Cubes`)))

(fn `SpawnSoundCube`
  (params (NbSoundCubes :type Integer) (CubeSpacing :type "Float (double-precision)"))
  (returns (SoundCubes :type "Array of /Game/Hibiki/03_Assets/Widget_Sound/BP_SoundCube Object Reference"))
  (bind (_returnvalue_x _returnvalue_y _returnvalue_z) (`KismetMathLibrary.BreakVector` (`SceneComponent.K2_GetComponentLocation` (`self.DefaultSceneRoot`))))
  ;[0.3439 1 0.8368 0.8] Spawn Audio Cubes
  (for _index (range 1 (+ NbSoundCubes 1))
    (bind _output_get (set `self.SpawnTransformLocationX` _returnvalue_x))
    (bind _output_get_2 (set `self.SpawnTransformLocationY` _returnvalue_y))
    ;[0.15 0.1367 0.04366 0.5] Modulate Orientation
    (if (`self.IsAxeX`)
      (if (`self.ReverseOrientation`)
        (bind _returnvalue (* _index CubeSpacing))
        (set `self.SpawnTransformLocationX` (+ _output_get _returnvalue))
        (else
          (set `self.SpawnTransformLocationX` (- _output_get _returnvalue))))
      (elif (`self.ReverseOrientation`)
        (set `self.SpawnTransformLocationY` (+ _output_get_2 _returnvalue))
        (else
          (set `self.SpawnTransformLocationY` (- _output_get_2 _returnvalue)))))
    (`|SpawnActorFromClass` "/Game/Hibiki/03_Assets/Widget_Sound/BP_SoundCube.BP_SoundCube_C" (`KismetMathLibrary.MakeTransform` (`KismetMathLibrary.MakeVector` (`self.SpawnTransformLocationX`) (`self.SpawnTransformLocationY`) _returnvalue_z) (struct) (0.1 0.1 0.1)) "Undefined" "MultiplyWithRoot" null null))
  ;[0.1749 0.2147 0.5565] Return an array of all spawned Cubes
  (bind _outactors (`GameplayStatics.GetAllActorsOfClass` "/Game/Hibiki/03_Assets/Widget_Sound/BP_SoundCube.BP_SoundCube_C"))
  (return _outactors))

(fn `SynesthesiaScaleSoundCube`
  (params (MusicDuration :type "Float (double-precision)") (PercentagePlayed :type "Float (double-precision)") (SoundCubes :type "Array of /Game/Hibiki/03_Assets/Widget_Sound/BP_SoundCube Object Reference"))
  (locals (FrequencyBandStrenths :type "Array of Float (single-precision)") (NewLocalVar :type "Float (double-precision)" :default 0.0))
  (bind _frequencybandstrenths (`local.FrequencyBandStrenths`))
  (bind _gameplaycamera (`self.GameplayCamera`))
  (bind _audiobeatprogression (`self.AudioBeatProgression`))
  (`|ExecutionSequence`
    (:`then_0`
      (set `self.PositionInAudio` (* MusicDuration PercentagePlayed)))
    (:`then_1`
      (set `local.FrequencyBandStrenths` (`ConstantQNRT.GetNormalizedChannelConstantQAtTime` (`self.SynesthesiaAnalysis`) (`self.PositionInAudio`) 0)))
    (:`then_2`
      (for (_array_element _array_index) _frequencybandstrenths
        (bind _cube (`/Game/Hibiki/03_Assets/Widget_Sound/BP_SoundCube.Cube` (`|GetArrayItem` SoundCubes _array_index)))
        (bind (_returnvalue_x _returnvalue_y _returnvalue_z) (`KismetMathLibrary.BreakVector` (`SceneComponent.K2_GetComponentScale` _cube)))
        (`SceneComponent.SetWorldScale3D` _cube (`KismetMathLibrary.MakeVector` _returnvalue_x _returnvalue_y (`KismetMathLibrary.Lerp` _returnvalue_z (* _array_element (`self.ScalingFactor`)) 0.5)))
        (`/Engine/EditorBlueprintResources/StandardMacros.IsValid` _gameplaycamera
          (:`Is Valid`
            (if (and (< _audiobeatprogression 0.75) (> _audiobeatprogression 0.25))
              (set `self.Threshold` 0.0)
              (else
                (set `self.Threshold` 1.0)))
            (`CameraComponent.SetFieldOfView` (`self.GetComponentByClass` _gameplaycamera "/Script/Engine.CameraComponent") (`KismetMathLibrary.Lerp` 45.0 (+ (* (`KismetMathLibrary.FClamp` (`|GetArrayItem` _frequencybandstrenths) 0.0 0.3) -1.0) 45.0) (`self.Threshold`)))))))))

(fn `UserConstructionScript`)