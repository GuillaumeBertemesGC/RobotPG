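; Audio visualiser actor that plays a music track and animates a row of spawned BP_SoundCube actors to its frequencies.
; BeginPlay spawns the cubes along X or Y, then collects every BP_SoundCube in the level into an array.
; Playback-percent updates sample pre-analysed Synesthesia Constant-Q bands, easing each cube's Z scale toward its band strength.
; The same loop sets an optional gameplay camera's FOV, so the last band determines it.
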(event `self.ReceiveBeginPlay`
  (bind _music (`self.Music`))
  (`|ExecutionSequence`
    (:`then_0`
      (`AudioComponent.SetSound` (`self.Audio`) _music)
      (set `self.MusicDuration` (`SoundBase.Duration` _music)))
    (:`then_1`
      (bind _soundcubes (`self.SpawnSoundCube` (`self.Nb Sound Cubes`) (`self.Cube Spacing`)))
      (set `self.Sound Cubes` _soundcubes))
    (:`then_2`
      (add `AudioComponent.OnAudioPlaybackPercent` (`self.Audio`) (delegate `OnPlayBackChange`)))
    (:`then_3`
      (`AudioComponent.Play` (`self.Audio`) 0.0))))

(event `OnPlayBackChange`
  (params (PlayingSoundWave :type "SoundWave Object Reference") (PlaybackPercent :type "Float (single-precision)"))
  (`self.SynesthesiaScaleSoundCube` (`self.MusicDuration`) PlaybackPercent (`self.Sound Cubes`)))

(fn `SpawnSoundCube`
  (params (NbSoundCubes :type Integer) (CubeSpacing :type "Float (double-precision)"))
  (returns (SoundCubes :type "Array of /Game/Hibiki/03_Assets/Widget_Sound/BP_SoundCube Object Reference"))
  (bind (_returnvalue_x _returnvalue_y _returnvalue_z) (`KismetMathLibrary.BreakVector` (`SceneComponent.K2_GetComponentLocation` (`self.DefaultSceneRoot`))))
  ;[0.3439 1 0.8368 0.8] Spawn Audio Cubes
  (for _index (range 1 (+ NbSoundCubes 1))
    (bind _output_get (set `self.SpawnTransformLocationX` _returnvalue_x))
    (bind _output_get_2 (set `self.SpawnTransformLocationY` _returnvalue_y))
    ;[0.15 0.1367 0.04366 0.5] Modulate Orientation
    (if (`self.IsAxeX`)
      (if (`self.ReverseOrientation`)
        (bind _returnvalue (* _index CubeSpacing))
        (set `self.SpawnTransformLocationX` (+ _output_get _returnvalue))
        (else
          (set `self.SpawnTransformLocationX` (- _output_get _returnvalue))))
      (elif (`self.ReverseOrientation`)
        (set `self.SpawnTransformLocationY` (+ _output_get_2 _returnvalue))
        (else
          (set `self.SpawnTransformLocationY` (- _output_get_2 _returnvalue)))))
    (`|SpawnActorFromClass` "/Game/Hibiki/03_Assets/Widget_Sound/BP_SoundCube.BP_SoundCube_C" (`KismetMathLibrary.MakeTransform` (`KismetMathLibrary.MakeVector` (`self.SpawnTransformLocationX`) (`self.SpawnTransformLocationY`) _returnvalue_z) (struct) (0.1 0.1 0.1)) "Undefined" "MultiplyWithRoot" null null))
  ;[0.1749 0.2147 0.5565] Return an array of all spawned Cubes
  (bind _outactors (`GameplayStatics.GetAllActorsOfClass` "/Game/Hibiki/03_Assets/Widget_Sound/BP_SoundCube.BP_SoundCube_C"))
  (return _outactors))

(fn `SynesthesiaScaleSoundCube`
  (params (MusicDuration :type "Float (double-precision)") (PercentagePlayed :type "Float (double-precision)") (SoundCubes :type "Array of /Game/Hibiki/03_Assets/Widget_Sound/BP_SoundCube Object Reference"))
  (locals (FrequencyBandStrenths :type "Array of Float (single-precision)"))
  (bind _gameplaycamera (`self.GameplayCamera`))
  (`|ExecutionSequence`
    (:`then_0`
      (set `self.PositionInAudio` (* MusicDuration PercentagePlayed)))
    (:`then_1`
      (set `local.FrequencyBandStrenths` (`ConstantQNRT.GetNormalizedChannelConstantQAtTime` (`self.SynesthesiaAnalysis`) (`self.PositionInAudio`) 0)))
    (:`then_2`
      (for (_array_element _array_index) (`local.FrequencyBandStrenths`)
        (bind _cube (`/Game/Hibiki/03_Assets/Widget_Sound/BP_SoundCube.Cube` (`|GetArrayItem` SoundCubes _array_index)))
        (bind (_returnvalue_x _returnvalue_y _returnvalue_z) (`KismetMathLibrary.BreakVector` (`SceneComponent.K2_GetComponentScale` _cube)))
        (bind _returnvalue (* _array_element (`self.ScalingFactor`)))
        (`SceneComponent.SetWorldScale3D` _cube (`KismetMathLibrary.MakeVector` _returnvalue_x _returnvalue_y (`KismetMathLibrary.Lerp` _returnvalue_z _returnvalue 0.5)))
        (`/Engine/EditorBlueprintResources/StandardMacros.IsValid` _gameplaycamera
          (:`Is Valid`
            (`CameraComponent.SetFieldOfView` (`self.GetComponentByClass` _gameplaycamera "/Script/Engine.CameraComponent") (+ (* _returnvalue 15.0) 35.0))))))))

(fn `UserConstructionScript`)