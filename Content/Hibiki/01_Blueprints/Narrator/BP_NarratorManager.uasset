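; Narrator manager that plays narration sequences as on-screen text with optional 2D voice audio, including win or loss narration after combat.
; Each line updates a lazily created widget, spawns its sound and sets a timer from the line or sound duration to pace the sequence.
; Starting a sequence interrupts any current one.
; After-battle narration reads the GameInstance's combat data and result, then clears that data if narration is enabled.
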(event `self.ReceiveBeginPlay`
  (`self.EnsureWidget`)
  (bind _ascontext (cast `/Game/Hibiki/01_Blueprints/SceneManagement/Context` (`GameplayStatics.GetGameInstance`)))
  (set `self.GameInstanceRef` _ascontext))

(fn `AdvanceLine`
  (bind _activesequence (`self.ActiveSequence`))
  (`/Engine/EditorBlueprintResources/StandardMacros.IncrementInt` (`self.CurrentLineIndex`)
    (:`  `
      (if (and (`KismetSystemLibrary.IsValid` _activesequence) (`KismetArrayLibrary.Array_IsValidIndex` (`/Game/Hibiki/01_Blueprints/Narrator/BP_NarratorDataType.Lines` _activesequence) (`self.CurrentLineIndex`)))
        (`self.ShowCurrentLine`)
        (else
          (`self.FinishNarration`))))))

(fn `EnsureWidget`
  (if (or (not (`KismetSystemLibrary.IsValidClass` (`self.NarratorWidgetClass`))) (`KismetSystemLibrary.IsValid` (`self.WidgetInstance`)))
    (return)
    (else
      (`/Engine/EditorBlueprintResources/StandardMacros.IsValid` (`GameplayStatics.GetPlayerController` 0)
        (:`Is Valid`
          (bind _returnvalue (`|CreateWidget` (`self.NarratorWidgetClass`) (`GameplayStatics.GetPlayerController` 0)))
          (set `self.WidgetInstance` _returnvalue)
          (bind _widgetinstance (`self.WidgetInstance`)
            (:`then`
              (`UserWidget.AddToViewport` _widgetinstance 50)
              (`Widget.SetVisibility` _widgetinstance "Hidden"))
            (:`else`)))
        (:`Is Not Valid`
          (return))))))

(fn `FinishNarration`
  (`KismetSystemLibrary.K2_ClearAndInvalidateTimerHandle` (`self.NarrationTimerHandle`))
  (`self.StopCurrentVoice`)
  (bind _widgetinstance (`self.WidgetInstance`)
    (:`then`
      (`Widget.SetVisibility` _widgetinstance "Hidden"))
    (:`else`
      _))
  (set `self.ActiveSequence` null)
  (set `self.CurrentLineIndex` 0))

(fn `PlayAfterBattleNarration`
  (bind _gameinstanceref (`self.GameInstanceRef`)
    (:`then`
      (bind _currentcombatdata (`/Game/Hibiki/01_Blueprints/SceneManagement/Context.CurrentCombatData` _gameinstanceref)
        (:`then`
          (if (`/Game/Hibiki/01_Blueprints/Battle/Data/BP_DA_CombatConfig.PlayNarration` _currentcombatdata)
            (if (`/Game/Hibiki/01_Blueprints/SceneManagement/Context.Succedeed` _gameinstanceref)
              (`self.PlayNarration` (`/Game/Hibiki/01_Blueprints/Battle/Data/BP_DA_CombatConfig.OnWinNarrationData` _currentcombatdata))
              (else
                (`self.PlayNarration` (`/Game/Hibiki/01_Blueprints/Battle/Data/BP_DA_CombatConfig.OnLossNarrationData` _currentcombatdata))))
            (set `/Game/Hibiki/01_Blueprints/SceneManagement/Context.CurrentCombatData` null _gameinstanceref)))
        (:`else`)))
    (:`else`)))

(fn `PlayDefaultNarration`
  (`self.PlayNarration` (`self.DefaultSequence`)))

(fn `PlayNarration`
  (params (Sequence :type "/Game/Hibiki/01_Blueprints/Narrator/BP_NarratorDataType Object Reference"))
  (`self.StopNarration`)
  (if (or (not (`KismetSystemLibrary.IsValid` Sequence)) (== (`KismetArrayLibrary.Array_Length` (`/Game/Hibiki/01_Blueprints/Narrator/BP_NarratorDataType.Lines` Sequence)) 0))
    (return)
    (else
      (set `self.ActiveSequence` (`local.Sequence`))
      (set `self.CurrentLineIndex` 0)
      (`self.EnsureWidget`)
      (`self.ShowCurrentLine`))))

(fn `ShowCurrentLine`
  (locals (CurrentLine :type "/Game/Hibiki/01_Blueprints/Narrator/FNarratorLine Structure") (SafeDuration :type "Float (double-precision)") (SoundDuration :type "Float (double-precision)" :default 0.1) (LineDuration :type "Float (double-precision)" :default 0.1))
  (bind _activesequence (`self.ActiveSequence`))
  (bind (_text _duration _voicesound _volume _pitch _usesoundduration) (break `/Game/Hibiki/01_Blueprints/Narrator/FNarratorLine` (`local.CurrentLine`)))
  (if (or (not (`KismetSystemLibrary.IsValid` _activesequence)) (not (`KismetArrayLibrary.Array_IsValidIndex` (`/Game/Hibiki/01_Blueprints/Narrator/BP_NarratorDataType.Lines` _activesequence) (`self.CurrentLineIndex`))))
    (`self.FinishNarration`)
    (return)
    (else
      (`self.EnsureWidget`)
      (bind _widgetinstance (`self.WidgetInstance`)
        (:`then`
          (bind _output_get (set `local.CurrentLine` (`|GetArrayItem` (`/Game/Hibiki/01_Blueprints/Narrator/BP_NarratorDataType.Lines` (`self.ActiveSequence`)) (`self.CurrentLineIndex`))))
          (bind (_text_2 _duration_2 _voicesound_2 _volume_2 _pitch_2) (break `/Game/Hibiki/01_Blueprints/Narrator/FNarratorLine` _output_get))
          (`/Game/Hibiki/01_Blueprints/Narrator/WB_NarratorBox.SetNarratorText` _widgetinstance _text_2)
          (`Widget.SetVisibility` _widgetinstance "HitTestInvisible")
          (`self.StopCurrentVoice`)
          (if (`KismetSystemLibrary.IsValid` _voicesound_2)
            (bind _returnvalue (`GameplayStatics.SpawnSound2D` _voicesound_2 _volume_2 _pitch_2 0.0 null))
            (set `self.CurrentVoiceAudio` _returnvalue))
          (set `local.LineDuration` _duration)
          (if (and (`KismetSystemLibrary.IsValid` _voicesound) _usesoundduration)
            (bind _output_get_2 (set `local.SoundDuration` (`SoundBase.Duration` _voicesound)))
            (if (> _output_get_2 0.0)
              (set `local.LineDuration` (`local.SoundDuration`))))
          (set `local.SafeDuration` (`KismetMathLibrary.FMax` (`local.LineDuration`) 0.1))
          (bind _returnvalue_2 (`KismetSystemLibrary.K2_SetTimerDelegate` (`|CreateDelegate` :!event `AdvanceLine`) (`local.SafeDuration`)))
          (set `self.NarrationTimerHandle` _returnvalue_2))
        (:`else`
          (return))))))

(fn `StopCurrentVoice`
  (bind _currentvoiceaudio (`self.CurrentVoiceAudio`)
    (:`then`
      (`AudioComponent.Stop` _currentvoiceaudio)
      (set `self.CurrentVoiceAudio` null))
    (:`else`)))

(fn `StopNarration`
  (`KismetSystemLibrary.K2_ClearAndInvalidateTimerHandle` (`self.NarrationTimerHandle`))
  (`self.StopCurrentVoice`)
  (bind _widgetinstance (`self.WidgetInstance`)
    (:`then`
      (`Widget.SetVisibility` _widgetinstance "Hidden"))
    (:`else`
      _))
  (set `self.ActiveSequence` null)
  (set `self.CurrentLineIndex` 0))

(fn `UserConstructionScript`)