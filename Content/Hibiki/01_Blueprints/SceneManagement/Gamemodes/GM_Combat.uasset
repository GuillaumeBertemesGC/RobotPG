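; GM_Combat is the combat game mode that handles screen transitions into combat and back out to the exploration level.
; On BeginPlay it plays a fade-out level sequence with movement and look input disabled, restoring state when finished.
; FadeIn plays a second input-locking sequence and binds an event to its completion.
; OpenExploLevel adds a black fade widget to the viewport, then opens the exploration level by object reference.
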(event `self.ReceiveBeginPlay`
  (`self.FadeOut`))

(event `OpenExploLevel`
  (bind _returnvalue (`|CreateWidget` "/Game/Hibiki/01_Blueprints/UI/WB_BlackFade.WB_BlackFade_C" (`GameplayStatics.GetPlayerController` 0)))
  (`UserWidget.AddToViewport` _returnvalue 0)
  (`GameplayStatics.OpenLevelBySoftObjectPtr` (`self.ExploLevel`)))

(fn `FadeIn`
  (bind (_outactor _returnvalue) (`LevelSequencePlayer.CreateLevelSequencePlayer` (`self.FadeInSequence`) (make `MovieSceneSequencePlaybackSettings` false (struct) (struct :`bAllowRounding` true) 1.0 0.0 false true true)))
  (add `MovieSceneSequencePlayer.OnFinished` _returnvalue (`|CreateDelegate` :!event `OpenExploLevel`))
  (`MovieSceneSequencePlayer.Play` _returnvalue))

(fn `FadeOut`
  (bind (_outactor _returnvalue) (`LevelSequencePlayer.CreateLevelSequencePlayer` (`self.FadeOutSequence`) (make `MovieSceneSequencePlaybackSettings` false (struct) (struct :`bAllowRounding` true) 1.0 0.0 false true true false false false "ForceRestoreState")))
  (`MovieSceneSequencePlayer.Play` _returnvalue))

(fn `UserConstructionScript`)