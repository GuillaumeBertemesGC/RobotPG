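; Exploration game mode that sets up the player's arrival in the level and provides the transition into the battle level behind a black fade widget.
; On BeginPlay it reads the Context game instance to play an intro, normal or after-loss spawn sequence, saving once the first launch is consumed.
; It teleports the player to the saved checkpoint or pending NPC transform, and caches checkpoints, doors and the narrator, with ID lookups for checkpoints and doors.
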(event `self.ReceiveBeginPlay`
  (`self.GetGameInstanceRef`)
  (`self.PlaySpawnSequence`)
  (`self.GetAllCheckpoints`)
  (`self.SetPlayerTransform`)
  (`self.GetAllDoors`)
  (`self.GetNarratorRef`))

(event `OpenBattleLevel`
  (bind _returnvalue (`|CreateWidget` "/Game/Hibiki/01_Blueprints/UI/WB_BlackFade.WB_BlackFade_C" (`GameplayStatics.GetPlayerController` 0)))
  (`UserWidget.AddToViewport` _returnvalue 0)
  (`GameplayStatics.OpenLevelBySoftObjectPtr` (`self.BattleLevel`)))

(fn `FadeIn`
  (bind (_outactor _returnvalue) (`LevelSequencePlayer.CreateLevelSequencePlayer` (`self.FadeInSequence`) (make `MovieSceneSequencePlaybackSettings` false (struct) (struct :`bAllowRounding` true) 1.0 0.0 false true true)))
  (add `MovieSceneSequencePlayer.OnFinished` _returnvalue (`|CreateDelegate` :!event `OpenBattleLevel`))
  (`MovieSceneSequencePlayer.Play` _returnvalue))

(fn `FadeOut`
  (bind (_outactor _returnvalue) (`LevelSequencePlayer.CreateLevelSequencePlayer` (`self.FadeOutSequence`) (make `MovieSceneSequencePlaybackSettings` false (struct) (struct :`bAllowRounding` true) 1.0 0.0 false true true false false false "ForceRestoreState")))
  (`MovieSceneSequencePlayer.Play` _returnvalue))

(fn `GetAllCheckpoints`
  (bind _outactors (`GameplayStatics.GetAllActorsOfClass` "/Game/Hibiki/01_Blueprints/Actors/BP_CheckPoint.BP_CheckPoint_C"))
  (set `self.Checkpoints` _outactors))

(fn `GetAllDoors`
  (bind _outactors (`GameplayStatics.GetAllActorsOfClass` "/Game/Hibiki/01_Blueprints/Actors/BP_Door.BP_Door_C"))
  (set `self.Doors` _outactors))

(fn `GetCheckpointTransform`
  (params (CheckpointId :type Name))
  (returns (CheckpointTransform :type "Transform Structure"))
  (locals (Checkpoint :type "Transform Structure"))
  (for _array_element (`self.Checkpoints`)
    (if (== (`/Game/Hibiki/01_Blueprints/Actors/BP_CheckPoint.CheckpointID` _array_element) CheckpointId)
      (set `local.Checkpoint` (`/Game/Hibiki/01_Blueprints/Actors/BP_CheckPoint.GetSpawnPoint` _array_element))
      (break)))
  (return (`local.Checkpoint`)))

(fn `GetDoorID`
  (params (DoorID :type Name))
  (returns (Door_Result :type "/Game/Hibiki/01_Blueprints/Actors/BP_Door Object Reference"))
  (if (`KismetArrayLibrary.Array_IsNotEmpty` (`self.Doors`))
    (for _array_element (`self.Doors`)
      (if (== (`/Game/Hibiki/01_Blueprints/Actors/BP_Door.DoorID` _array_element) DoorID)
        (return _array_element))))
  (return null))

(fn `GetGameInstanceRef`
  (bind _ascontext (cast `/Game/Hibiki/01_Blueprints/SceneManagement/Context` (`GameplayStatics.GetGameInstance`)))
  (set `self.GameInstanceRef` _ascontext))

(fn `GetNarratorRef`
  (bind _returnvalue (`GameplayStatics.GetActorOfClass` "/Game/Hibiki/01_Blueprints/Narrator/BP_NarratorManager.BP_NarratorManager_C"))
  (set `self.NarratorRef` _returnvalue))

(fn `PlayClassicSpawn`
  (bind (_outactor _returnvalue) (`LevelSequencePlayer.CreateLevelSequencePlayer` "/Game/Hibiki/08_Sequences/LS_SpawnCheckpoint.LS_SpawnCheckpoint" (make `MovieSceneSequencePlaybackSettings` false (struct) (struct :`bAllowRounding` true) 1.0 0.0 false true true false false false "ForceRestoreState")))
  (`MovieSceneSequencePlayer.Play` _returnvalue))

(fn `PlayIntroSequence`
  (bind (_outactor _returnvalue) (`LevelSequencePlayer.CreateLevelSequencePlayer` "/Game/Hibiki/08_Sequences/LS_Intro.LS_Intro" (make `MovieSceneSequencePlaybackSettings` false (struct) (struct :`bAllowRounding` true) 1.0 0.0 false true true false false false "ForceRestoreState")))
  (`MovieSceneSequencePlayer.Play` _returnvalue))

(fn `PlayOnLossSpawn`
  (bind (_outactor _returnvalue) (`LevelSequencePlayer.CreateLevelSequencePlayer` "/Game/Hibiki/08_Sequences/LS_SpawnCheckpointAfterLose.LS_SpawnCheckpointAfterLose" (make `MovieSceneSequencePlaybackSettings` false (struct) (struct :`bAllowRounding` true) 1.0 0.0 false true true false false false "ForceRestoreState")))
  (`MovieSceneSequencePlayer.Play` _returnvalue))

(fn `PlaySpawnSequence`
  (bind _gameinstanceref (`self.GameInstanceRef`)
    (:`then`
      (if (`/Game/Hibiki/01_Blueprints/SceneManagement/Context.FirstLaunch?` _gameinstanceref)
        (`self.PlayIntroSequence`)
        (set `/Game/Hibiki/01_Blueprints/SceneManagement/Context.FirstLaunch?` false _gameinstanceref)
        (`/Game/Hibiki/01_Blueprints/SceneManagement/Context.SaveAllDatas` _gameinstanceref)
        (elif (`/Game/Hibiki/01_Blueprints/SceneManagement/Context.Succedeed` _gameinstanceref)
          (`self.PlayClassicSpawn`)
          (else
            (`self.PlayOnLossSpawn`)))))
    (:`else`)))

(fn `SetPlayerTransform`
  (bind _returnvalue (`GameplayStatics.GetPlayerCharacter` 0))
  (bind _ascontext (cast `/Game/Hibiki/01_Blueprints/SceneManagement/Context` (`GameplayStatics.GetGameInstance`)))
  (if (`/Game/Hibiki/01_Blueprints/SceneManagement/Context.bShouldSpawnOnNPC?` _ascontext)
    (bind (_pendingnpccheckpointtransform_location _pendingnpccheckpointtransform_rotation) (`KismetMathLibrary.BreakTransform` (`/Game/Hibiki/01_Blueprints/SceneManagement/Context.PendingNPCCheckpointTransform` _ascontext)))
    (`self.K2_SetActorTransform` (`GameplayStatics.GetPlayerCharacter` 0) (`KismetMathLibrary.MakeTransform` _pendingnpccheckpointtransform_location _pendingnpccheckpointtransform_rotation) false true)
    (set `/Game/Hibiki/01_Blueprints/SceneManagement/Context.bShouldSpawnOnNPC?` false _ascontext)
    (else
      (`/Engine/EditorBlueprintResources/StandardMacros.IsValid` _returnvalue
        (:`Is Valid`
          (bind (_checkpointtransform_location _checkpointtransform_rotation) (`KismetMathLibrary.BreakTransform` (`self.GetCheckpointTransform` (`/Game/Hibiki/01_Blueprints/SceneManagement/Context.CurrentCheckpointId` _ascontext))))
          (`self.K2_SetActorTransform` _returnvalue (`KismetMathLibrary.MakeTransform` _checkpointtransform_location _checkpointtransform_rotation) false true))))))

(fn `UserConstructionScript`)