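; PC_Combat is a player controller, named for combat, that toggles the pause menu.
; The IA_Pause input checks whether a stored WB_PauseMenu is on screen.
; If so, it removes and clears the widget, restores game-only input, hides the cursor and unpauses.
; Otherwise it creates a fresh menu, focuses it with game-and-UI input, shows the cursor and pauses the game.
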(event `EnhancedInput|/Game/Hibiki/04_Inputs/Actions/IA_Pause`
  (params (ActionValue :type Boolean) (ElapsedSeconds :type "Float (double-precision)") (TriggeredSeconds :type "Float (double-precision)") (InputAction :type "InputAction Object Reference" :default "/Game/Hibiki/04_Inputs/Actions/IA_Pause.IA_Pause"))
  (:`Started`
    (bind _pausemenuref (`self.PauseMenuRef`)
      (:`then`
        (if (`Widget.IsInViewport` _pausemenuref)
          (`Widget.RemoveFromParent` _pausemenuref)
          (set `self.PauseMenuRef` null)
          (`WidgetBlueprintLibrary.SetInputMode_GameOnly` self)
          (set `self.bShowMouseCursor` false)
          (`GameplayStatics.SetGamePaused` false)
          (else
            (bind _returnvalue (`|CreateWidget` "/Game/Hibiki/01_Blueprints/UI/WB_PauseMenu.WB_PauseMenu_C" self :!label _label))
            (set `self.PauseMenuRef` _returnvalue)
            (`UserWidget.AddToViewport` _returnvalue 0)
            (`WidgetBlueprintLibrary.SetInputMode_GameAndUIEx` self _returnvalue)
            (set `self.bShowMouseCursor` true)
            (`GameplayStatics.SetGamePaused` true))))
      (:`else`
        (goto _label)))))

(fn `UserConstructionScript`)