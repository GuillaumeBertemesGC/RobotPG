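; Sliding double door to a boss area that opens for the player and starts the boss theme the first time it is triggered.
; BeginPlay clears the lock if DoorID is among the save game's unlocked doors, and otherwise tints the lights red; events swap red and green visuals.
; When unlocked, entering the box plays a Timeline sliding both panels apart; leaving only plays the opening sound, with no closing motion.
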(event `self.ReceiveBeginPlay`
  (bind _ascontext (cast `/Game/Hibiki/01_Blueprints/SceneManagement/Context` (`GameplayStatics.GetGameInstance`))
    (:`then`
      (bind _output_get (set `self.GameInstanceRef` _ascontext))
      (bind _currentsavegame (`/Game/Hibiki/01_Blueprints/SceneManagement/Context.CurrentSaveGame` _output_get)
        (:`then`
          (bind _unlockeddoorids (`/Game/Hibiki/01_Blueprints/SceneManagement/Save/BP_SaveGame.UnlockedDoorIDs` _currentsavegame))
          (if (`KismetArrayLibrary.Array_IsNotEmpty` _unlockeddoorids)
            (if (`KismetArrayLibrary.Array_Contains` _unlockeddoorids (`self.DoorID`))
              (set `self.bIsLock` false))))
        (:`else`
          _)))
    (:`CastFailed`
      _))
  (set `self.LeftDoorClosePos` (`SceneComponent.RelativeLocation` (`self.SM_Door_Left`)))
  (set `self.RightDoorClosePos` (`SceneComponent.RelativeLocation` (`self.SM_Door_Right`)))
  (if (`self.bIsLock`)
    (`PrimitiveComponent.SetMaterial` (`self.SM_Door_Left`) 1 "/Game/SciFi_BioLaboratory/Materials/Objects/MI_Light_Red.MI_Light_Red")
    (`PrimitiveComponent.SetMaterial` (`self.SM_Door_Left`) 2 "/Game/SciFi_BioLaboratory/Materials/Objects/MI_Light_Red.MI_Light_Red")
    (`PrimitiveComponent.SetMaterial` (`self.SM_Door_Right`) 1 "/Game/SciFi_BioLaboratory/Materials/Objects/MI_Light_Red.MI_Light_Red")))

(event `self.Box.OnComponentBeginOverlap`
  (params (OverlappedComponent :type "PrimitiveComponent Object Reference") (OtherActor :type "Actor Object Reference") (OtherComp :type "PrimitiveComponent Object Reference") (OtherBodyIndex :type Integer) (bFromSweep :type Boolean) (SweepResult :type "HitResult Structure (by ref)"))
  (bind _leftdoorclosepos (`self.LeftDoorClosePos`))
  (bind _rightdoorclosepos (`self.RightDoorClosePos`))
  (bind _returnvalue (`KismetMathLibrary.MakeVector` (`self.SideDistance`)))
  (cast `/Game/Hibiki/01_Blueprints/Characters/BP_PlayerCharacter` OtherActor)
  (if (`self.bIsLock`)
    _
    (elif (`self.IsBossThemePlayed`)
      (bind (_direction _newtrack_0) (`Timeline|Timeline` :!label _label)
        (:`Update`
          (`SceneComponent.K2_SetRelativeLocation` (`self.SM_Door_Left`) (`KismetMathLibrary.VLerp` _leftdoorclosepos (- _leftdoorclosepos _returnvalue) _newtrack_0) false false)
          (`SceneComponent.K2_SetRelativeLocation` (`self.SM_Door_Right`) (`KismetMathLibrary.VLerp` _rightdoorclosepos (+ _rightdoorclosepos _returnvalue) _newtrack_0) false false)))
      (else
        (`GameplayStatics.PlaySound2D` "/Game/Hibiki/03_Assets/Widget_Sound/Unlike_Pluto_-_Everything_Black__feat__Mike_Taylor.Unlike_Pluto_-_Everything_Black__feat__Mike_Taylor" 1.0 1.0 0.0 null null)
        (set `self.IsBossThemePlayed` true)
        (goto _label)))))

(event `self.Box.OnComponentEndOverlap`
  (params (OverlappedComponent :type "PrimitiveComponent Object Reference") (OtherActor :type "Actor Object Reference") (OtherComp :type "PrimitiveComponent Object Reference") (OtherBodyIndex :type Integer))
  (cast `/Game/Hibiki/01_Blueprints/Characters/BP_PlayerCharacter` OtherActor)
  (if (not (`self.bIsLock`))
    (`self.PlaySFX` (`self.SFX_DoorOpening`))))

(event `SetDoorUnlockVisual`
  (`PrimitiveComponent.SetMaterial` (`self.SM_Door_Left`) 1 "/Game/SciFi_BioLaboratory/Materials/Objects/MI_Light_Green.MI_Light_Green")
  (`PrimitiveComponent.SetMaterial` (`self.SM_Door_Left`) 2 "/Game/SciFi_BioLaboratory/Materials/Objects/MI_Light_Green.MI_Light_Green")
  (`PrimitiveComponent.SetMaterial` (`self.SM_Door_Right`) 1 "/Game/SciFi_BioLaboratory/Materials/Objects/MI_Light_Green.MI_Light_Green"))

(event `SetDoorLockVisual`
  (`PrimitiveComponent.SetMaterial` (`self.SM_Door_Left`) 1 "/Game/SciFi_BioLaboratory/Materials/Objects/MI_Light_Red.MI_Light_Red")
  (`PrimitiveComponent.SetMaterial` (`self.SM_Door_Left`) 2 "/Game/SciFi_BioLaboratory/Materials/Objects/MI_Light_Red.MI_Light_Red")
  (`PrimitiveComponent.SetMaterial` (`self.SM_Door_Right`) 1 "/Game/SciFi_BioLaboratory/Materials/Objects/MI_Light_Red.MI_Light_Red"))

(fn `PlaySFX`
  (params (Sound :type "SoundBase Object Reference"))
  (bind (_returnvalue_x _returnvalue_y _returnvalue_z) (`KismetMathLibrary.BreakVector` (`SceneComponent.K2_GetComponentLocation` (`self.SM_Door_Left`))))
  (`GameplayStatics.PlaySoundAtLocation` Sound (`KismetMathLibrary.MakeVector` _returnvalue_x _returnvalue_y (+ _returnvalue_z 100.0)) (struct) 1.0 1.0 0.0 (`self.SoundAttenuation`) null self null))

(fn `UserConstructionScript`)