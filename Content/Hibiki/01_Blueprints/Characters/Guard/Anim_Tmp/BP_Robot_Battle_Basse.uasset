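; Battle robot actor for the Guard character that relays left and right shooting to its arm animation and carries a Niagara effect.
; Each shoot event casts the anim instance to ABP_Guard_Arm_Location and passes it the note location.
; The IsOpportunities flag selects the plain shoot call when true and the O variant when false.
; Every tick, the Niagara component snaps to the world position of the mesh's ALL bone.
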(event `self.ReceiveTick`
  (params (DeltaSeconds :type "Float (single-precision)"))
  (bind _returnvalue_location (`KismetMathLibrary.BreakTransform` (`SkinnedMeshComponent.GetBoneTransform` (`self.SkeletalMesh`) "ALL" "RTS_World")))
  (`SceneComponent.K2_SetWorldLocation` (`self.Niagara`) _returnvalue_location false false))

(event `Left_Shoot_O`
  (params (IsOpportunities :type Boolean) (Note_Location :type "Vector Structure"))
  (bind _asabp_guard_arm_location (cast `/Game/Hibiki/01_Blueprints/Characters/Guard/Anim_Tmp/ABP_Guard_Arm_Location` (`SkeletalMeshComponent.GetAnimInstance` (`self.SkeletalMesh`))))
  (if IsOpportunities
    (`/Game/Hibiki/01_Blueprints/Characters/Guard/Anim_Tmp/ABP_Guard_Arm_Location.Left_Shoot` _asabp_guard_arm_location Note_Location)
    (else
      (`/Game/Hibiki/01_Blueprints/Characters/Guard/Anim_Tmp/ABP_Guard_Arm_Location.Left_Shoot_O` _asabp_guard_arm_location Note_Location))))

(event `Right_Shoot_O`
  (params (IsOpportunities :type Boolean) (`Note Location` :type "Vector Structure"))
  (bind _asabp_guard_arm_location (cast `/Game/Hibiki/01_Blueprints/Characters/Guard/Anim_Tmp/ABP_Guard_Arm_Location` (`SkeletalMeshComponent.GetAnimInstance` (`self.SkeletalMesh`))))
  (if IsOpportunities
    (`/Game/Hibiki/01_Blueprints/Characters/Guard/Anim_Tmp/ABP_Guard_Arm_Location.Right_Shoot` _asabp_guard_arm_location `Note Location`)
    (else
      (`/Game/Hibiki/01_Blueprints/Characters/Guard/Anim_Tmp/ABP_Guard_Arm_Location.Right_Shoot_O` _asabp_guard_arm_location `Note Location`))))

(fn `UserConstructionScript`)