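; Guard NPC that shows a name label, hides itself if the save lists it as defeated, and saves its linked checkpoint when interacted with.
; On BeginPlay, guards using the guard animation bob the mesh via a timeline started at a random time.
; Overlapping characters trigger head look-at through an AnimBP alpha and make the label yaw toward them.
; Interactible state scales the label in and out, and closing conversations notifies the instigator.
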(event `self.ReceiveBeginPlay`
  ; Idle
  (bind _ascontext (cast `/Game/Hibiki/01_Blueprints/SceneManagement/Context` (`GameplayStatics.GetGameInstance`))
    (:`then`
      (bind _output_get (set `self.GameInstanceRef` _ascontext))
      (bind _currentsavegame (`/Game/Hibiki/01_Blueprints/SceneManagement/Context.CurrentSaveGame` _output_get)
        (:`then`
          (bind _defeatednpcids (`/Game/Hibiki/01_Blueprints/SceneManagement/Save/BP_SaveGame.DefeatedNPCIDs` _currentsavegame))
          (if (`KismetArrayLibrary.Array_IsNotEmpty` _defeatednpcids)
            (bind _output_get_2 (set `self.bDefeated` (`KismetArrayLibrary.Array_Contains` _defeatednpcids (`self.NPCID`))))
            (if _output_get_2
              (`self.SetActorHiddenInGame` true)
              (`self.SetActorEnableCollision` false)
              (else
                (set `self.Relative Location` (`SceneComponent.RelativeLocation` (`self.Mesh`)) :!label _label)
                (if (`self.UseGuardAnim`)
                  (`self.SetRandomStartAnim`)
                  (bind (_direction _axisymovement) (`Timeline|TL_LocationZ`)
                    (:`Update`
                      (`SceneComponent.K2_SetRelativeLocation` (`self.Mesh`) (+ (`self.Relative Location`) _axisymovement) false false))))))
            (else
              (goto _label))))
        (:`else`
          (goto _label))))
    (:`CastFailed`
      (goto _label))))

(event `PlayGuardAnim`
  (params (Anim :type "/Game/Hibiki/01_Blueprints/Characters/Guard/E_Guard_Anim Enum" :default "NewEnumerator0"))
  (set `self.CurrentAnimation` Anim))

(event `self.ReceiveTick`
  (params (DeltaSeconds :type "Float (single-precision)"))
  (bind _txt_charactername (`self.Txt_CharacterName`))
  (bind _targetactor (`self.TargetActor`))
  (bind (_returnvalue_roll _returnvalue_pitch _returnvalue_yaw) (`KismetMathLibrary.BreakRotator` (`KismetMathLibrary.FindLookAtRotation` (`SceneComponent.K2_GetComponentLocation` _txt_charactername) (`SceneComponent.K2_GetComponentLocation` (`Actor.RootComponent` _targetactor)))))
  (if (`self.IsPlayerInRange`)
    ; Look At Text
    (`/Engine/EditorBlueprintResources/StandardMacros.IsValid` _targetactor
      (:`Is Valid`
        (`SceneComponent.K2_SetRelativeRotation` _txt_charactername (`KismetMathLibrary.MakeRotator` 0.0 0.0 (+ _returnvalue_yaw 180.0)) false false)))))

(event `self.ReceiveActorBeginOverlap`
  (params (OtherActor :type "Actor Object Reference"))
  (bind _ascharacter (cast `Character` OtherActor))
  (set `self.TargetActor` _ascharacter)
  (set `self.IsPlayerInRange` true)
  ; Enable Look At Head
  (bind _asabp_guard_looking_at_player (cast `/Game/Hibiki/03_Assets/Mesh/Guard/ABP_Guard_LookingAtPlayer` (`SkeletalMeshComponent.GetAnimInstance` (`self.Mesh`))))
  (bind (_direction _newtrack_0) (`Timeline|LookAt` :!via `PlayFromStart`)
    (:`Update`
      (set `/Game/Hibiki/03_Assets/Mesh/Guard/ABP_Guard_LookingAtPlayer.LookAtAlpha` _newtrack_0 _asabp_guard_looking_at_player))))

(event `self.ReceiveActorEndOverlap`
  (params (OtherActor :type "Actor Object Reference"))
  (set `self.IsPlayerInRange` false)
  ; Disable Look At Head
  (bind _asabp_guard_looking_at_player (cast `/Game/Hibiki/03_Assets/Mesh/Guard/ABP_Guard_LookingAtPlayer` (`SkeletalMeshComponent.GetAnimInstance` (`self.Mesh`))))
  (bind (_direction _newtrack_0) (`Timeline|LookAt2` :!via `ReverseFromEnd`)
    (:`Update`
      (set `/Game/Hibiki/03_Assets/Mesh/Guard/ABP_Guard_LookingAtPlayer.LookAtAlpha` _newtrack_0 _asabp_guard_looking_at_player))))

(event `/Game/Hibiki/01_Blueprints/Interfaces/BP_Interactiblee.SetInteractibleState`
  (params (`bCanSowInteract?` :type Boolean))
  (bind _txt_charactername (`self.Txt_CharacterName`))
  (bind _txt_charactername_2 (`self.Txt_CharacterName`))
  (if `bCanSowInteract?`
    (`SceneComponent.SetVisibility` _txt_charactername_2 true false)
    (bind (_direction _newtrack_0) (`Timeline|TextOn` :!via `PlayFromStart`)
      (:`Update`
        (`SceneComponent.SetRelativeScale3D` _txt_charactername_2 (`KismetMathLibrary.Conv_DoubleToVector` _newtrack_0))))
    (else
      (bind (_direction_2 _newtrack_0_2) (`Timeline|Text Off` :!via `PlayFromStart`)
        (:`Update`
          (`SceneComponent.SetRelativeScale3D` _txt_charactername (`KismetMathLibrary.Conv_DoubleToVector` _newtrack_0_2)))
        (:`Finished`
          (`SceneComponent.SetVisibility` _txt_charactername false false))))))

(event `/Game/Hibiki/01_Blueprints/Interfaces/BP_Interactiblee.ConversationClosed`
  (message `/Game/Hibiki/01_Blueprints/Interfaces/BP_Interactiblee.ConversationClosed` (`self.InteractInstigator`)))

(event `/Game/Hibiki/01_Blueprints/Interfaces/BP_Interactiblee.Interact`
  (params (Instigator :type "Actor Object Reference"))
  (`self.SaveLinkedCheckpointId`))

(fn `SaveLinkedCheckpointId`
  (bind _gameinstanceref (`self.GameInstanceRef`)
    (:`then`
      (bind _output_get (set `/Game/Hibiki/01_Blueprints/SceneManagement/Context.CurrentCheckpointId` (`self.LinkedCheckpointId`) _gameinstanceref))
      (`/Game/Hibiki/01_Blueprints/SceneManagement/Context.SaveCheckpointId` _gameinstanceref _output_get))
    (:`else`)))

(fn `SetRandomStartAnim`
  (locals (NewTimeRandom :type "Float (double-precision)"))
  (bind _output_get (set `local.NewTimeRandom` (`KismetMathLibrary.RandomFloatInRange` 0.0 5.0)))
  (`TimelineComponent.SetNewTime` (`self.TL_LocationZ`) _output_get))

(fn `UserConstructionScript`
  (`TextRenderComponent.K2_SetText` (`self.Txt_CharacterName`) (`self.CharacterName`)))