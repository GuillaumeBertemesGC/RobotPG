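; Guard NPC that shows its name and, on interaction, saves its linked checkpoint ID through the game instance.
; BeginPlay hides it and disables collision if the save lists it as defeated, otherwise starts randomly offset idle timelines for body, head and arms.
; Further timelines play Happy or Disappointed reactions on these separate parts.
; Character overlap eases the head toward that character, Tick keeps tracking, and end overlap runs a return timeline.
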(event `self.ReceiveBeginPlay`
  ; Idle
  (bind _ascontext (cast `/Game/Hibiki/01_Blueprints/SceneManagement/Context` (`GameplayStatics.GetGameInstance`))
    (:`then`
      (bind _output_get (set `self.GameInstanceRef` _ascontext))
      (bind _currentsavegame (`/Game/Hibiki/01_Blueprints/SceneManagement/Context.CurrentSaveGame` _output_get)
        (:`then`
          (bind _defeatednpcids (`/Game/Hibiki/01_Blueprints/SceneManagement/Save/BP_SaveGame.DefeatedNPCIDs` _currentsavegame))
          (if (`KismetArrayLibrary.Array_IsNotEmpty` _defeatednpcids)
            (bind _output_get_2 (set `self.bDefeated` (`KismetArrayLibrary.Array_Contains` _defeatednpcids (`self.NPCID`))))
            (if _output_get_2
              (`self.SetActorHiddenInGame` true)
              (`self.SetActorEnableCollision` false)
              (else
                (`self.SetRandomStartAnim` :!label _label)
                (`|ExecutionSequence`
                  (:`then_0`
                    (bind (_direction _axisymovement) (`Timeline|Timeline`)
                      (:`Update`
                        (`SceneComponent.K2_SetRelativeLocation` (`self.Mesh`) _axisymovement false false))))
                  (:`then_1`
                    (bind (_direction_2 _axisymovement_2) (`Timeline|Timeline_2`)
                      (:`Update`
                        (`SceneComponent.K2_SetRelativeLocation` (`self.Tete_002`) _axisymovement_2 false false))))
                  (:`then_2`
                    (bind (_direction_3 _axisyxmovement) (`Timeline|Timeline_0`)
                      (:`Update`
                        (`SceneComponent.K2_SetRelativeLocation` (`self.Bras_gauche_001`) _axisyxmovement false false))))
                  (:`then_3`
                    (bind (_direction_4 _axisyxmovement_2) (`Timeline|Timeline_1`)
                      (:`Update`
                        (`SceneComponent.K2_SetRelativeLocation` (`self.Bras_droit_001`) _axisyxmovement_2 false false)))))))
            (else
              (goto _label))))
        (:`else`
          (goto _label))))
    (:`CastFailed`
      (goto _label))))

(event `PlayGuardAnim`
  (params (Anim :type "/Game/Hibiki/01_Blueprints/Characters/Guard/E_Guard_Anim Enum" :default "NewEnumerator0"))
  (set `self.CurrentAnimation` Anim)
  (`self.Anim`))

(event `Anim`
  (bind _mesh (`self.Mesh`))
  (bind _mesh_2 (`self.Mesh`))
  (bind _bras_gauche_001 (`self.Bras_gauche_001`))
  (bind _bras_droit_001 (`self.Bras_droit_001`))
  (bind _relativelocation (`SceneComponent.RelativeLocation` _mesh))
  (bind _relativelocation_2 (`SceneComponent.RelativeLocation` _bras_droit_001))
  (bind _relativelocation_3 (`SceneComponent.RelativeLocation` _mesh_2))
  (bind _relativelocation_4 (`SceneComponent.RelativeLocation` _bras_gauche_001))
  (switch `/Game/Hibiki/01_Blueprints/Characters/Guard/E_Guard_Anim` (`self.CurrentAnimation`)
    (:`NewEnumerator1`
      (`|ExecutionSequence`
        (:`then_0`
          (bind (_direction _happytrack) (`Timeline|TL_HappyAnim` :!via `PlayFromStart`)
            (:`Update`
              (`SceneComponent.K2_SetRelativeLocation` _mesh_2 (`KismetMathLibrary.VLerp` _relativelocation_3 (+ _relativelocation_3 (0.0 0.0 30.0)) _happytrack) true false))))
        (:`then_1`
          (bind (_direction_2 _happytrack_2) (`Timeline|TL_HappyAnim_Arms` :!via `PlayFromStart`)
            (:`Update`
              (`|ExecutionSequence`
                (:`then_0`
                  (bind _returnvalue (* _happytrack_2 360.0))
                  (`SceneComponent.K2_SetRelativeRotation` (`self.Bras_gauche_001`) (`KismetMathLibrary.MakeRotator` 0.0 0.0 _returnvalue) false false))
                (:`then_1`
                  (`SceneComponent.K2_SetRelativeRotation` (`self.Bras_droit_001`) (`KismetMathLibrary.MakeRotator` 0.0 0.0 _returnvalue) false false))))))))
    (:`NewEnumerator2`
      (bind (_direction_3 _happytrack_3) (`Timeline|TL_Disapointed` :!via `PlayFromStart`)
        (:`Update`
          (`|ExecutionSequence`
            (:`then_0`
              (`SceneComponent.K2_SetRelativeLocation` _mesh (`KismetMathLibrary.VLerp` _relativelocation (+ _relativelocation (0.0 0.0 -20.0)) _happytrack_3) true false))
            (:`then_1`
              (`SceneComponent.K2_SetRelativeLocation` _bras_gauche_001 (`KismetMathLibrary.VLerp` _relativelocation_4 (+ _relativelocation_4 (0.0 0.0 -20.0)) _happytrack_3) true false))
            (:`then_2`
              (`SceneComponent.K2_SetRelativeLocation` _bras_droit_001 (`KismetMathLibrary.VLerp` _relativelocation_2 (+ _relativelocation_2 (0.0 0.0 -20.0)) _happytrack_3) true false))))))))

(event `self.ReceiveTick`
  (params (DeltaSeconds :type "Float (single-precision)"))
  (bind _tete_002 (`self.Tete_002`))
  (bind _targetactor (`self.TargetActor`))
  (bind (_returnvalue_roll _returnvalue_pitch _returnvalue_yaw) (`KismetMathLibrary.BreakRotator` (`KismetMathLibrary.FindLookAtRotation` (`SceneComponent.K2_GetComponentLocation` _tete_002) (`SceneComponent.K2_GetComponentLocation` (`Actor.RootComponent` _targetactor)))))
  (if (`self.IsPlayerInRange`)
    (`/Engine/EditorBlueprintResources/StandardMacros.IsValid` _targetactor
      (:`Is Valid`
        (`SceneComponent.K2_SetRelativeRotation` _tete_002 (`KismetMathLibrary.MakeRotator` 0.0 0.0 (+ _returnvalue_yaw 180.0)) false false)))))

(event `self.ReceiveActorBeginOverlap`
  (params (OtherActor :type "Actor Object Reference"))
  (bind _targetactor (`self.TargetActor`))
  (bind (_returnvalue_roll _returnvalue_pitch _returnvalue_yaw) (`KismetMathLibrary.BreakRotator` (`KismetMathLibrary.FindLookAtRotation` (`SceneComponent.K2_GetComponentLocation` (`self.Tete_002`)) (`SceneComponent.K2_GetComponentLocation` (`Actor.RootComponent` _targetactor)))))
  (bind _ascharacter (cast `Character` OtherActor))
  (set `self.TargetActor` _ascharacter)
  (bind (_direction _happytrack) (`Timeline|TL_Start_Head` :!via `PlayFromStart`)
    (:`Update`
      (`/Engine/EditorBlueprintResources/StandardMacros.IsValid` _targetactor
        (:`Is Valid`
          (`SceneComponent.K2_SetRelativeRotation` (`self.Tete_002`) (`KismetMathLibrary.MakeRotator` 0.0 0.0 (* (+ _returnvalue_yaw 180.0) _happytrack)) false false))))
    (:`Finished`
      (set `self.IsPlayerInRange` true))))

(event `self.ReceiveActorEndOverlap`
  (params (OtherActor :type "Actor Object Reference"))
  (bind _tete_002 (`self.Tete_002`))
  (bind (_relativerotation_roll _relativerotation_pitch _relativerotation_yaw) (`KismetMathLibrary.BreakRotator` (`SceneComponent.RelativeRotation` _tete_002)))
  (set `self.IsPlayerInRange` false)
  (bind (_direction _happytrack) (`Timeline|TL_Return_Head` :!via `PlayFromStart`)
    (:`Update`
      (`SceneComponent.K2_SetRelativeRotation` _tete_002 (`KismetMathLibrary.MakeRotator` 0.0 0.0 (* _relativerotation_yaw _happytrack)) false false)
      (set `self.TargetActor` null))))

(event `/Game/Hibiki/01_Blueprints/Interfaces/BP_Interactiblee.SetInteractibleState`
  (params (`bCanSowInteract?` :type Boolean))
  (if `bCanSowInteract?`
    (`SceneComponent.SetVisibility` (`self.Txt_CharacterName`) true false)
    (else
      (`SceneComponent.SetVisibility` (`self.Txt_CharacterName`) false false))))

(event `/Game/Hibiki/01_Blueprints/Interfaces/BP_Interactiblee.ConversationClosed`
  (message `/Game/Hibiki/01_Blueprints/Interfaces/BP_Interactiblee.ConversationClosed` (`self.InteractInstigator`)))

(event `/Game/Hibiki/01_Blueprints/Interfaces/BP_Interactiblee.Interact`
  (params (Instigator :type "Actor Object Reference"))
  (`self.SaveLinkedCheckpointId`))

(fn `Anim_Happy`)

(fn `SaveLinkedCheckpointId`
  (bind _gameinstanceref (`self.GameInstanceRef`)
    (:`then`
      (bind _output_get (set `/Game/Hibiki/01_Blueprints/SceneManagement/Context.CurrentCheckpointId` (`self.LinkedCheckpointId`) _gameinstanceref))
      (`/Game/Hibiki/01_Blueprints/SceneManagement/Context.SaveCheckpointId` _gameinstanceref _output_get))
    (:`else`)))

(fn `SetRandomStartAnim`
  (locals (NewTimeRandom :type "Float (double-precision)"))
  (bind _newtimerandom (`local.NewTimeRandom`))
  (bind _output_get (set `local.NewTimeRandom` (`KismetMathLibrary.RandomFloatInRange` 0.0 5.0)))
  (`TimelineComponent.SetNewTime` (`self.Timeline`) _output_get)
  (`TimelineComponent.SetNewTime` (`self.Timeline_0`) _newtimerandom)
  (`TimelineComponent.SetNewTime` (`self.Timeline_1`) _newtimerandom)
  (`TimelineComponent.SetNewTime` (`self.Timeline_2`) _newtimerandom))

(fn `UserConstructionScript`
  (`TextRenderComponent.K2_SetText` (`self.Txt_CharacterName`) (`self.CharacterName`)))