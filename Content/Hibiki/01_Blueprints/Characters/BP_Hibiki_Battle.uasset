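; Battle Blueprint for the Hibiki player robot, relaying arm attacks aimed at note locations to its animation Blueprint.
; Left and right arm events cast the skeletal mesh's anim instance to ABP_Hibiki_Battle and call the matching StarShoot with the note location.
; The IsStarShoot flag has no effect, as the CircleBattery calls are disconnected.
; Tick moves a Niagara effect to the BoneEffect_end bone each frame.
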(event `self.ReceiveTick`
  (params (DeltaSeconds :type "Float (single-precision)"))
  (bind _returnvalue_location (`KismetMathLibrary.BreakTransform` (`SkinnedMeshComponent.GetBoneTransform` (`self.SK_PlayerRobot`) "BoneEffect_end" "RTS_World")))
  (`SceneComponent.K2_SetWorldLocation` (`self.Niagara`) (+ _returnvalue_location (0.0 0.0 0.0)) false false))

(event `Hibiki_Left_Arm`
  (params (IsStarShoot :type Boolean) (NoteLocation :type "Vector Structure"))
  (bind _asabp_hibiki_battle (cast `/Game/Hibiki/01_Blueprints/Characters/ABP_Hibiki_Battle` (`SkeletalMeshComponent.GetAnimInstance` (`self.SK_PlayerRobot`))))
  (if IsStarShoot
    _
    (else
      _))
  (`/Game/Hibiki/01_Blueprints/Characters/ABP_Hibiki_Battle.Left_StarShoot` _asabp_hibiki_battle NoteLocation))

(event `Hibiki_Right_Arm`
  (params (IsStarShoot :type Boolean) (NoteLocation :type "Vector Structure"))
  (bind _asabp_hibiki_battle (cast `/Game/Hibiki/01_Blueprints/Characters/ABP_Hibiki_Battle` (`SkeletalMeshComponent.GetAnimInstance` (`self.SK_PlayerRobot`))))
  (if IsStarShoot
    _
    (else
      _))
  (`/Game/Hibiki/01_Blueprints/Characters/ABP_Hibiki_Battle.Right_StarShoot` _asabp_hibiki_battle NoteLocation))

(fn `UserConstructionScript`)