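; BP_TriggerNarration is a trigger volume that starts a narration when the player character enters its box.
; It finds the BP_NarratorManager on BeginPlay and passes its NarrationData to that manager's PlayNarration.
; An overlap is ignored while the manager has an active sequence.
; Once a narration has been sent, HasTriggered blocks repeats unless CanRetrigger is set.
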(event `self.ReceiveBeginPlay`
  (bind _returnvalue (`GameplayStatics.GetActorOfClass` "/Game/Hibiki/01_Blueprints/Narrator/BP_NarratorManager.BP_NarratorManager_C"))
  (set `self.NarratorManagerRef` _returnvalue))

(event `self.Box.OnComponentBeginOverlap`
  (params (OverlappedComponent :type "PrimitiveComponent Object Reference") (OtherActor :type "Actor Object Reference") (OtherComp :type "PrimitiveComponent Object Reference") (OtherBodyIndex :type Integer) (bFromSweep :type Boolean) (SweepResult :type "HitResult Structure (by ref)"))
  (cast `/Game/Hibiki/01_Blueprints/Characters/BP_PlayerCharacter` OtherActor)
  (if (not (`self.IsNarratorPlaying`))
    (if (not (`self.HasTriggered`))
      (`self.PlayNarration`)
      (elif (`self.CanRetrigger`)
        (`self.PlayNarration`)))))

(fn `IsNarratorPlaying`
  (returns (ReturnValue :type Boolean))
  (bind _narratormanagerref (`self.NarratorManagerRef`)
    (:`then`
      (bind _activesequence (`/Game/Hibiki/01_Blueprints/Narrator/BP_NarratorManager.ActiveSequence` _narratormanagerref)
        (:`then`
          (return (`KismetSystemLibrary.IsValid` _activesequence)))
        (:`else`
          _)))
    (:`else`
      _))
  (return false))

(fn `PlayNarration`
  (bind _narratormanagerref (`self.NarratorManagerRef`)
    (:`then`
      (bind _narrationdata (`self.NarrationData`)
        (:`then`
          (`/Game/Hibiki/01_Blueprints/Narrator/BP_NarratorManager.PlayNarration` _narratormanagerref _narrationdata)
          (set `self.HasTriggered` true))
        (:`else`
          _)))
    (:`else`
      _))
  (return))

(fn `UserConstructionScript`)