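; BP_TriggerMusic is a box trigger volume that switches the game's music while the player's third-person character is inside it.
; BeginPlay caches the Context game instance, which handles the music requests.
; Overlap begin requests the NewMusic track with a short fade, saving the current one as previous.
; Overlap end asks the game instance to fade back to that previous music.
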(event `self.ReceiveBeginPlay`
  (bind _ascontext (cast `/Game/Blueprints/Context` (`GameplayStatics.GetGameInstance`)))
  (set `self.GameInstanceRef` _ascontext))

(event `self.Box.OnComponentBeginOverlap`
  (params (OverlappedComponent :type "PrimitiveComponent Object Reference") (OtherActor :type "Actor Object Reference") (OtherComp :type "PrimitiveComponent Object Reference") (OtherBodyIndex :type Integer) (bFromSweep :type Boolean) (SweepResult :type "HitResult Structure (by ref)"))
  (cast `/Game/ThirdPerson/Blueprints/BP_ThirdPersonCharacter` OtherActor)
  (bind _gameinstanceref (`self.GameInstanceRef`)
    (:`then`
      (`/Game/Blueprints/Context.RequestMusic` _gameinstanceref (`self.New Music`) 1.0 true))
    (:`else`)))

(event `self.Box.OnComponentEndOverlap`
  (params (OverlappedComponent :type "PrimitiveComponent Object Reference") (OtherActor :type "Actor Object Reference") (OtherComp :type "PrimitiveComponent Object Reference") (OtherBodyIndex :type Integer))
  (cast `/Game/ThirdPerson/Blueprints/BP_ThirdPersonCharacter` OtherActor)
  (bind _gameinstanceref (`self.GameInstanceRef`)
    (:`then`
      (`/Game/Blueprints/Context.ReturnToPreviousMusic` _gameinstanceref 1.0))
    (:`else`)))

(fn `UserConstructionScript`)