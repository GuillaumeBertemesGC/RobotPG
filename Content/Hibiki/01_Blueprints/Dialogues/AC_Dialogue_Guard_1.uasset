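; Dialogue component for a guard that raises an intruder alert and damages the player when spoken to.
; It overrides the parent Dialogue function and, on the first tree node, shows a "Mouse" speaker line with a single Continue option.
; Once that line passes through, it casts the player to BP_ThirdPersonCharacter, applies damage, clears dialogue progress and closes the conversation.
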(fn `Dialogue`
  (`parent.Dialogue`)
  (switch `int` (`self.DialogueTreeIndex`)
    (:`0`
      (bind _state (`self.AddDialogue` "Mouse" "BIP BOUP \n!!ALERTE INTRUE!!" (`|MakeArray` "Continue" :!type "Text")))
      (switch `/Game/Hibiki/01_Blueprints/Dialogues/Enum_DialogueState` _state
        (:`NewEnumerator0`
          (bind _asbp_third_person_character (cast `/Game/ThirdPerson/Blueprints/BP_ThirdPersonCharacter` (`GameplayStatics.GetPlayerCharacter` 0)))
          (`GameplayStatics.ApplyDamage` _asbp_third_person_character 10.0)
          (`self.ClearDialogueProgress`)
          (`self.CloseConversation` false))))))