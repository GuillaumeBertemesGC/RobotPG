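; Dialogue component for the guard boss Ange-0016, who renames himself Daniel and reluctantly lets the silent player go on, warning in French of harder challenges ahead.
; It overrides Dialogue, calls the parent, then runs tree index 0 as a linear chain of AddDialogue calls advanced on Pass Through.
; Every line shares one audio asset and a single "..." reply.
; The final line clears dialogue progress and closes the conversation.
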(fn `Dialogue`
  (`parent.Dialogue`)
  (switch `int` (`self.DialogueTreeIndex`)
    (:`0`
      (bind _state (`self.AddDialogue` "Ange-0016" "Hum..." (`|MakeArray` "..." :!type "Text") "/Game/Hibiki/07_Sfx/Guard_Boss1.Guard_Boss1"))
      (switch `/Game/Hibiki/01_Blueprints/Dialogues/Enum_DialogueState` _state
        (:`NewEnumerator0`
          (bind _state_2 (`self.AddDialogue` "Ange-0016" "Je me disais bien qu'un autre petit frère finirais par venir jusqu'a moi." (`|MakeArray` "..." :!type "Text") "/Game/Hibiki/07_Sfx/Guard_Boss1.Guard_Boss1"))
          (switch `/Game/Hibiki/01_Blueprints/Dialogues/Enum_DialogueState` _state_2
            (:`NewEnumerator0`
              (bind _state_3 (`self.AddDialogue` "Ange-0016" "Appelle moi Daniel, c'est un matricule Humain." (`|MakeArray` "..." :!type "Text") "/Game/Hibiki/07_Sfx/Guard_Boss1.Guard_Boss1"))
              (switch `/Game/Hibiki/01_Blueprints/Dialogues/Enum_DialogueState` _state_3
                (:`NewEnumerator0`
                  (bind _state_4 (`self.AddDialogue` "Daniel" "ça fait sont effet!" (`|MakeArray` "..." :!type "Text") "/Game/Hibiki/07_Sfx/Guard_Boss1.Guard_Boss1"))
                  (switch `/Game/Hibiki/01_Blueprints/Dialogues/Enum_DialogueState` _state_4
                    (:`NewEnumerator0`
                      (bind _state_5 (`self.AddDialogue` "Daniel" "Non?" (`|MakeArray` "..." :!type "Text") "/Game/Hibiki/07_Sfx/Guard_Boss1.Guard_Boss1"))
                      (switch `/Game/Hibiki/01_Blueprints/Dialogues/Enum_DialogueState` _state_5
                        (:`NewEnumerator0`
                          (bind _state_6 (`self.AddDialogue` "Daniel" "..." (`|MakeArray` "..." :!type "Text") "/Game/Hibiki/07_Sfx/Guard_Boss1.Guard_Boss1"))
                          (switch `/Game/Hibiki/01_Blueprints/Dialogues/Enum_DialogueState` _state_6
                            (:`NewEnumerator0`
                              (bind _state_7 (`self.AddDialogue` "Daniel" "Tu ne parle pas?" (`|MakeArray` "..." :!type "Text") "/Game/Hibiki/07_Sfx/Guard_Boss1.Guard_Boss1"))
                              (switch `/Game/Hibiki/01_Blueprints/Dialogues/Enum_DialogueState` _state_7
                                (:`NewEnumerator0`
                                  (bind _state_8 (`self.AddDialogue` "Daniel" "Ok, je vois..." (`|MakeArray` "..." :!type "Text") "/Game/Hibiki/07_Sfx/Guard_Boss1.Guard_Boss1"))
                                  (switch `/Game/Hibiki/01_Blueprints/Dialogues/Enum_DialogueState` _state_8
                                    (:`NewEnumerator0`
                                      (bind _state_9 (`self.AddDialogue` "Daniel" "Tu peut rester avec moi si tu le souhaite." (`|MakeArray` "..." :!type "Text") "/Game/Hibiki/07_Sfx/Guard_Boss1.Guard_Boss1"))
                                      (switch `/Game/Hibiki/01_Blueprints/Dialogues/Enum_DialogueState` _state_9
                                        (:`NewEnumerator0`
                                          (bind _state_10 (`self.AddDialogue` "Daniel" "En tous cas, je te déconseille d'aller plus loin." (`|MakeArray` "..." :!type "Text") "/Game/Hibiki/07_Sfx/Guard_Boss1.Guard_Boss1"))
                                          (switch `/Game/Hibiki/01_Blueprints/Dialogues/Enum_DialogueState` _state_10
                                            (:`NewEnumerator0`
                                              (bind _state_11 (`self.AddDialogue` "Daniel" "Bon,.. tu m'a l'air déterminer..." (`|MakeArray` "..." :!type "Text") "/Game/Hibiki/07_Sfx/Guard_Boss1.Guard_Boss1"))
                                              (switch `/Game/Hibiki/01_Blueprints/Dialogues/Enum_DialogueState` _state_11
                                                (:`NewEnumerator0`
                                                  (bind _state_12 (`self.AddDialogue` "Daniel" "Tu peut y aller si tu veux." (`|MakeArray` "..." :!type "Text") "/Game/Hibiki/07_Sfx/Guard_Boss1.Guard_Boss1"))
                                                  (switch `/Game/Hibiki/01_Blueprints/Dialogues/Enum_DialogueState` _state_12
                                                    (:`NewEnumerator0`
                                                      (bind _state_13 (`self.AddDialogue` "Daniel" "Mais ATTENTION!" (`|MakeArray` "..." :!type "Text") "/Game/Hibiki/07_Sfx/Guard_Boss1.Guard_Boss1"))
                                                      (switch `/Game/Hibiki/01_Blueprints/Dialogues/Enum_DialogueState` _state_13
                                                        (:`NewEnumerator0`
                                                          (bind _state_14 (`self.AddDialogue` "Daniel" "Ce sera plus dur," (`|MakeArray` "..." :!type "Text") "/Game/Hibiki/07_Sfx/Guard_Boss1.Guard_Boss1"))
                                                          (switch `/Game/Hibiki/01_Blueprints/Dialogues/Enum_DialogueState` _state_14
                                                            (:`NewEnumerator0`
                                                              (bind _state_15 (`self.AddDialogue` "Daniel" "Bien plus dur." (`|MakeArray` "..." :!type "Text") "/Game/Hibiki/07_Sfx/Guard_Boss1.Guard_Boss1"))
                                                              (switch `/Game/Hibiki/01_Blueprints/Dialogues/Enum_DialogueState` _state_15
                                                                (:`NewEnumerator0`
                                                                  (`self.ClearDialogueProgress`)
                                                                  (`self.CloseConversation` true))))))))))))))))))))))))))))))))))