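; Dialogue component for the third guard tutorial, where the Overseer briefs the player on a final check before fighting without guidance.
; It overrides Dialogue, calls the parent, then branches on the dialogue tree index, with a single tree defined.
; That tree chains four French lines with one continue option and a shared voice cue.
; It ends by clearing dialogue progress and closing the conversation.
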(fn `Dialogue`
  (locals (Audio :type "SoundBase Soft Object Reference"))
  (bind _audio (`local.Audio`))
  (`parent.Dialogue`)
  (switch `int` (`self.DialogueTreeIndex`)
    (:`0`
      (bind _output_get (set `local.Audio` "/Game/Hibiki/07_Sfx/Overseer/SFX_Overseer_Voices_Cue.SFX_Overseer_Voices_Cue"))
      (bind _state (`self.AddDialogue` "OVERSEER" "Dernière vérification." (`|MakeArray` "..." :!type "Text") _output_get))
      (switch `/Game/Hibiki/01_Blueprints/Dialogues/Enum_DialogueState` _state
        (:`NewEnumerator0`
          (bind _state_2 (`self.AddDialogue` "OVERSEER" "Cette unité alternera attaques et ouvertures." (`|MakeArray` "...." :!type "Text") _audio))
          (switch `/Game/Hibiki/01_Blueprints/Dialogues/Enum_DialogueState` _state_2
            (:`NewEnumerator0`
              (bind _state_3 (`self.AddDialogue` "OVERSEER" "Aucune nouvelle mécanique." (`|MakeArray` "..." :!type "Text") _audio))
              (switch `/Game/Hibiki/01_Blueprints/Dialogues/Enum_DialogueState` _state_3
                (:`NewEnumerator0`
                  (bind _state_4 (`self.AddDialogue` "OVERSEER" "Je veux simplement voir ce que tu fais lorsque je cesse de te guider." (`|MakeArray` "..." :!type "Text") _audio))
                  (switch `/Game/Hibiki/01_Blueprints/Dialogues/Enum_DialogueState` _state_4
                    (:`NewEnumerator0`
                      (`self.ClearDialogueProgress`)
                      (`self.CloseConversation` true))))))))))))