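; Dialogue component for the second guard tutorial, in which the Overseer explains in French that enemy attacks appear as obstacles to dodge and lists the control keys.
; It overrides Dialogue, calls the parent, then switches on DialogueTreeIndex, with only the first branch defined.
; That branch chains AddDialogue lines through their Pass Through state with a shared voice cue, then clears progress and closes the conversation.
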(fn `Dialogue`
  (locals (Audio :type "SoundBase Soft Object Reference"))
  (bind _audio (`local.Audio`))
  (`parent.Dialogue`)
  (switch `int` (`self.DialogueTreeIndex`)
    (:`0`
      (bind _output_get (set `local.Audio` "/Game/Hibiki/07_Sfx/Overseer/SFX_Overseer_Voices_Cue.SFX_Overseer_Voices_Cue"))
      (bind _state (`self.AddDialogue` "OVERSEER" "Celui-ci possède une fonction offensive." (`|MakeArray` "..." :!type "Text") _output_get))
      (switch `/Game/Hibiki/01_Blueprints/Dialogues/Enum_DialogueState` _state
        (:`NewEnumerator0`
          (bind _state_2 (`self.AddDialogue` "OVERSEER" "Ses attaques apparaîtront sous forme d'obstacles" (`|MakeArray` "...." :!type "Text") _audio))
          (switch `/Game/Hibiki/01_Blueprints/Dialogues/Enum_DialogueState` _state_2
            (:`NewEnumerator0`
              (bind _state_3 (`self.AddDialogue` "OVERSEER" "Contrairement aux opportunités…" (`|MakeArray` "..." :!type "Text") _audio))
              (switch `/Game/Hibiki/01_Blueprints/Dialogues/Enum_DialogueState` _state_3
                (:`NewEnumerator0`
                  (bind _state_4 (`self.AddDialogue` "OVERSEER" "…ne les frappe pas. Esquive !" (`|MakeArray` "..." :!type "Text") _audio))
                  (switch `/Game/Hibiki/01_Blueprints/Dialogues/Enum_DialogueState` _state_4
                    (:`NewEnumerator0`
                      (bind _state_5 (`self.AddDialogue` "OVERSEER" "Tes commandes sont 'D' 'F' et 'J' 'K'." (`|MakeArray` "..." :!type "Text") _audio))
                      (switch `/Game/Hibiki/01_Blueprints/Dialogues/Enum_DialogueState` _state_5
                        (:`NewEnumerator0`
                          (`self.ClearDialogueProgress`)
                          (`self.CloseConversation` true))))))))))))))