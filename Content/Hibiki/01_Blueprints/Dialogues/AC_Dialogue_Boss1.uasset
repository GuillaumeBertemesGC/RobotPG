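; Dialogue component for the first boss, where the OVERSEER introduces a final trial against a more advanced unit, in French.
; It overrides Dialogue, calls the parent, then switches on DialogueTreeIndex, with only tree 0 defined.
; Single-option AddDialogue calls share one voice cue and chain through their Pass Through state.
; After the last AddDialogue call, it clears dialogue progress and closes the conversation.
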(fn `Dialogue`
  (locals (Audio :type "SoundBase Soft Object Reference"))
  (`parent.Dialogue`)
  (switch `int` (`self.DialogueTreeIndex`)
    (:`0`
      (set `local.Audio` "/Game/Hibiki/07_Sfx/Overseer/SFX_Overseer_Voices_Cue.SFX_Overseer_Voices_Cue")
      (bind _state (`self.AddDialogue` "OVERSEER" "J'ai préparé une dernière épreuve." (`|MakeArray` "..." :!type "Text") (`local.Audio`)))
      (switch `/Game/Hibiki/01_Blueprints/Dialogues/Enum_DialogueState` _state
        (:`NewEnumerator0`
          (bind _state_2 (`self.AddDialogue` "OVERSEER" "Une unité légèrement plus avancée." (`|MakeArray` "...." :!type "Text") (`local.Audio`)))
          (switch `/Game/Hibiki/01_Blueprints/Dialogues/Enum_DialogueState` _state_2
            (:`NewEnumerator0`
              (bind _state_3 (`self.AddDialogue` "OVERSEER" "J'ai ajusté ses paramètres selon tes performances précédentes." (`|MakeArray` "...." :!type "Text") (`local.Audio`)))
              (switch `/Game/Hibiki/01_Blueprints/Dialogues/Enum_DialogueState` _state_3
                (:`NewEnumerator0`
                  (bind _state_4 (`self.AddDialogue` "OVERSEER" "Et selon quelques données plus…" (`|MakeArray` "...." :!type "Text") (`local.Audio`)))
                  (switch `/Game/Hibiki/01_Blueprints/Dialogues/Enum_DialogueState` _state_4
                    (:`NewEnumerator0`
                      (bind _state_5 (`self.AddDialogue` "OVERSEER" "récentes." (`|MakeArray` "...." :!type "Text") (`local.Audio`)))
                      (switch `/Game/Hibiki/01_Blueprints/Dialogues/Enum_DialogueState` _state_5
                        (:`NewEnumerator0`
                          (bind _state_6 (`self.AddDialogue` "OVERSEER" "Purement scientifiques.." (`|MakeArray` "...." :!type "Text") (`local.Audio`)))
                          (switch `/Game/Hibiki/01_Blueprints/Dialogues/Enum_DialogueState` _state_6
                            (:`NewEnumerator0`
                              (bind _state_7 (`self.AddDialogue` "OVERSEER" "Tu connais les règles." (`|MakeArray` "...." :!type "Text") (`local.Audio`)))
                              (switch `/Game/Hibiki/01_Blueprints/Dialogues/Enum_DialogueState` _state_7
                                (:`NewEnumerator0`
                                  (bind _state_8 (`self.AddDialogue` "OVERSEER" "Opportunités." (`|MakeArray` "...." :!type "Text") (`local.Audio`)))
                                  (switch `/Game/Hibiki/01_Blueprints/Dialogues/Enum_DialogueState` _state_8
                                    (:`NewEnumerator0`
                                      (bind _state_9 (`self.AddDialogue` "OVERSEER" "Obstacles.." (`|MakeArray` "...." :!type "Text") (`local.Audio`)))
                                      (switch `/Game/Hibiki/01_Blueprints/Dialogues/Enum_DialogueState` _state_9
                                        (:`NewEnumerator0`
                                          (`self.AddDialogue` "OVERSEER" "Et essaye peut-être de rester concentré cette fois..." (`|MakeArray` "!" :!type "Text") (`local.Audio`))
                                          (`self.ClearDialogueProgress`)
                                          (`self.CloseConversation` true))))))))))))))))))))))