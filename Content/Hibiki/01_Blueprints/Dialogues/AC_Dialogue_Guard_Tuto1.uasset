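; Dialogue component for the first tutorial exercise, in which the OVERSEER explains in French the music-driven "opportunity" combat system and its keys.
; The Dialogue override calls its parent, then runs tree index 0 as a linear chain of voiced, single-option AddDialogue lines, each advancing on Pass Through.
; The final line sets a guard animation, then progress is cleared and the conversation closes.
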(fn `Dialogue`
  (`parent.Dialogue`)
  (switch `int` (`self.DialogueTreeIndex`)
    (:`0`
      (bind _state (`self.AddDialogue` "OVERSEER" "Premier exercice." (`|MakeArray` "..." :!type "Text") "/Game/Hibiki/07_Sfx/Overseer/SFX_Overseer_Voice_01.SFX_Overseer_Voice_01"))
      (switch `/Game/Hibiki/01_Blueprints/Dialogues/Enum_DialogueState` _state
        (:`NewEnumerator0`
          (bind _state_2 (`self.AddDialogue` "OVERSEER" "L'unité devant toi est désarmée." (`|MakeArray` "..." :!type "Text") "/Game/Hibiki/07_Sfx/Overseer/SFX_Overseer_Voice_02.SFX_Overseer_Voice_02"))
          (switch `/Game/Hibiki/01_Blueprints/Dialogues/Enum_DialogueState` _state_2
            (:`NewEnumerator0`
              (bind _state_3 (`self.AddDialogue` "OVERSEER" "Enfin…" (`|MakeArray` "..." :!type "Text") "/Game/Hibiki/07_Sfx/Overseer/SFX_Overseer_Voice_05.SFX_Overseer_Voice_05"))
              (switch `/Game/Hibiki/01_Blueprints/Dialogues/Enum_DialogueState` _state_3
                (:`NewEnumerator0`
                  (bind _state_4 (`self.AddDialogue` "OVERSEER" "Presque." (`|MakeArray` "..." :!type "Text") "/Game/Hibiki/07_Sfx/Overseer/SFX_Overseer_Voice_02.SFX_Overseer_Voice_02"))
                  (switch `/Game/Hibiki/01_Blueprints/Dialogues/Enum_DialogueState` _state_4
                    (:`NewEnumerator0`
                      (bind _state_5 (`self.AddDialogue` "OVERSEER" "Ton système de combat repose sur ce que j'appelle des opportunités.." (`|MakeArray` "..." :!type "Text") "/Game/Hibiki/07_Sfx/Overseer/SFX_Overseer_Voice_08.SFX_Overseer_Voice_08"))
                      (switch `/Game/Hibiki/01_Blueprints/Dialogues/Enum_DialogueState` _state_5
                        (:`NewEnumerator0`
                          (bind _state_6 (`self.AddDialogue` "OVERSEER" "Lorsque la musique et le comportement de ton adversaire créent une ouverture, ton interface la matérialisera.." (`|MakeArray` "..." :!type "Text") "/Game/Hibiki/07_Sfx/Overseer/SFX_Overseer_Voice_09.SFX_Overseer_Voice_09"))
                          (switch `/Game/Hibiki/01_Blueprints/Dialogues/Enum_DialogueState` _state_6
                            (:`NewEnumerator0`
                              (bind _state_7 (`self.AddDialogue` "OVERSEER" "Frappe au bon moment.." (`|MakeArray` "..." :!type "Text") "/Game/Hibiki/07_Sfx/Overseer/SFX_Overseer_Voice_02.SFX_Overseer_Voice_02"))
                              (switch `/Game/Hibiki/01_Blueprints/Dialogues/Enum_DialogueState` _state_7
                                (:`NewEnumerator0`
                                  (bind _state_8 (`self.AddDialogue` "OVERSEER" "Tes commantes sont 'R' 'E' et 'U' 'I'." (`|MakeArray` "..." :!type "Text") "/Game/Hibiki/07_Sfx/Overseer/SFX_Overseer_Voices_Cue.SFX_Overseer_Voices_Cue"))
                                  (switch `/Game/Hibiki/01_Blueprints/Dialogues/Enum_DialogueState` _state_8
                                    (:`NewEnumerator0`
                                      (bind _state_9 (`self.AddDialogue` "OVERSEER" "Bon entrainement." (`|MakeArray` "!" :!type "Text") "/Game/Hibiki/07_Sfx/Overseer/SFX_Overseer_Voice_04.SFX_Overseer_Voice_04" null "NewEnumerator3"))
                                      (switch `/Game/Hibiki/01_Blueprints/Dialogues/Enum_DialogueState` _state_9
                                        (:`NewEnumerator0`
                                          (`self.ClearDialogueProgress`)
                                          (`self.CloseConversation` true))))))))))))))))))))))