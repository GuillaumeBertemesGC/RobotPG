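; AC_MapLoader is a battle component that loads the current rhythm combat map's data from the Context game instance.
; LoadMap calls RetrieveConfig, which casts the game instance to Context and validates its CurrentCombatData.
; On success it stores the music track and BPM events, then appends every Opportunities and Obstacles DataTable row to matching arrays.
; On failure it only prints an error message.
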(event `LoadMap`
  (bind (_currentcombatdata _bsuccess) (`self.RetrieveConfig`))
  (if _bsuccess
    (`|ExecutionSequence`
      (:`then_0`
        (set `self.Track` (`/Game/Hibiki/01_Blueprints/Battle/Data/BP_DA_CombatConfig.MusicTrack` _currentcombatdata)))
      (:`then_1`
        (set `self.BPMEvents` (`/Game/Hibiki/01_Blueprints/Battle/Data/BP_DA_CombatConfig.BPMEvent` _currentcombatdata)))
      (:`then_2`
        (bind _opportunities (`/Game/Hibiki/01_Blueprints/Battle/Data/BP_DA_CombatConfig.Opportunities` _currentcombatdata))
        (bind _outrownames (`DataTableFunctionLibrary.GetDataTableRowNames` _opportunities))
        (for _array_element _outrownames
          (bind _returnvalue (`|GetDataTableRow` _opportunities _array_element)
            (:`then`
              (`KismetArrayLibrary.Array_Add` (`self.Opportunities`) _returnvalue)))))
      (:`then_3`
        (bind _obstacles (`/Game/Hibiki/01_Blueprints/Battle/Data/BP_DA_CombatConfig.Obstacles` _currentcombatdata))
        (bind _outrownames_2 (`DataTableFunctionLibrary.GetDataTableRowNames` _obstacles))
        (for _array_element_2 _outrownames_2
          (bind _returnvalue_2 (`|GetDataTableRow` _obstacles _array_element_2)
            (:`then`
              (`KismetArrayLibrary.Array_Add` (`self.Obstacles`) _returnvalue_2))))))
    (else
      (`KismetSystemLibrary.PrintString` "Retrieve Config Data failed." true true (struct :`R` 1.0 :`G` 0.003883 :`A` 1.0)))))

(fn `RetrieveConfig`
  (returns (CurrentCombatData :type "/Game/Hibiki/01_Blueprints/Battle/Data/BP_DA_CombatConfig Object Reference") (bSuccess :type Boolean))
  (bind _ascontext (cast `/Game/Blueprints/Context` (`GameplayStatics.GetGameInstance`))
    (:`then`
      (bind _currentcombatdata (`/Game/Blueprints/Context.CurrentCombatData` _ascontext)
        (:`then`
          (return _currentcombatdata true))
        (:`else`
          _)))
    (:`CastFailed`
      _))
  (return null false))