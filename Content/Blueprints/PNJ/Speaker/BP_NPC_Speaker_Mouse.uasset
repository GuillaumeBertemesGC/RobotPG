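; BP_NPC_Speaker_Mouse is an NPC speaker Blueprint that opens a conversation when interacted with.
; Interact stores the instigator, then calls OpenConversation on the ACDialogueMouse component.
; An unconnected chain that would play environment audio and pass it to a W_SoundVisualiser widget never runs.
; BeginPlay is empty, and the construction script only calls its parent.
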(event `self.ReceiveBeginPlay`)

(event `/Game/Hibiki/01_Blueprints/Interfaces/BP_Interactiblee.Interact`
  (params (Instigator :type "Actor Object Reference"))
  (set `self.InteractInstigator` Instigator)
  (`/Game/Hibiki/01_Blueprints/Dialogues/AC_Dialogue_Base.OpenConversation` (`self.AC_Dialogue_Mouse`)))

(fn `UserConstructionScript`
  (`parent.UserConstructionScript`))