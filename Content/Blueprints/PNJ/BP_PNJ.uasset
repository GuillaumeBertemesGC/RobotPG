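; NPC (PNJ) Blueprint that plays a one-time, line-by-line dialogue when the player interacts with it.
; Its InteractionSphere shows a prompt widget and sets the player's OnInteraction flag, which Tick checks when polling the E key.
; The first press disables player input and opens WB_MainDialogue; later presses advance DialogueText, then close it.
; Reaching the last line can trigger SceneLoaderRef, then unlock DoorToUnlock's visual and damage the player.
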(event `self.InteractionSphere.OnComponentBeginOverlap`
  (params (OverlappedComponent :type "PrimitiveComponent Object Reference") (OtherActor :type "Actor Object Reference") (OtherComp :type "PrimitiveComponent Object Reference") (OtherBodyIndex :type Integer) (bFromSweep :type Boolean) (SweepResult :type "HitResult Structure (by ref)"))
  ;[0.694 0.6979 0.189 0.5] Interaction Dialogue
  (cast `/Game/Hibiki/01_Blueprints/Characters/BP_PlayerCharacter` OtherActor)
  (bind _returnvalue (`|CreateWidget` "/Game/Hibiki/01_Blueprints/UI/WB_Interaction.WB_Interaction_C" (`GameplayStatics.GetPlayerController` 0)))
  (bind _output_get (set `self.UI_Interaction` _returnvalue))
  (`UserWidget.AddToViewport` _output_get 0)
  (bind _asbp_third_person_character (cast `/Game/Hibiki/01_Blueprints/Characters/BP_PlayerCharacter` (`GameplayStatics.GetPlayerCharacter` 0)))
  (set `/Game/Hibiki/01_Blueprints/Characters/BP_PlayerCharacter.bOnInteraction` true _asbp_third_person_character))

(event `self.InteractionSphere.OnComponentEndOverlap`
  (params (OverlappedComponent :type "PrimitiveComponent Object Reference") (OtherActor :type "Actor Object Reference") (OtherComp :type "PrimitiveComponent Object Reference") (OtherBodyIndex :type Integer))
  (bind _ui_interaction (`self.UI_Interaction`))
  ;[0.694 0.6979 0.189 0.5] Interaction Dialogue
  (cast `/Game/Hibiki/01_Blueprints/Characters/BP_PlayerCharacter` OtherActor)
  (`/Engine/EditorBlueprintResources/StandardMacros.IsValid` _ui_interaction
    (:`Is Valid`
      (`Widget.RemoveFromParent` _ui_interaction)
      (bind _asbp_third_person_character (cast `/Game/Hibiki/01_Blueprints/Characters/BP_PlayerCharacter` (`GameplayStatics.GetPlayerCharacter` 0)))
      (set `/Game/Hibiki/01_Blueprints/Characters/BP_PlayerCharacter.bOnInteraction` false _asbp_third_person_character))))

(event `self.ReceiveTick`
  (params (DeltaSeconds :type "Float (single-precision)"))
  (bind _doortounlock (`self.DoorToUnlock`))
  (bind _dialoguetext (`self.DialogueText`))
  (bind _dialogueindex (`self.DialogueIndex`))
  (bind _ui_maindialogue (`self.UI_MainDialogue`))
  (bind _returnvalue (`KismetArrayLibrary.Array_Length` _dialoguetext))
  (if (`PlayerController.WasInputKeyJustPressed` (`GameplayStatics.GetPlayerController` 0) "E")
    (bind _asbp_third_person_character (cast `/Game/Hibiki/01_Blueprints/Characters/BP_PlayerCharacter` (`GameplayStatics.GetPlayerCharacter` 0)))
    (if (`/Game/Hibiki/01_Blueprints/Characters/BP_PlayerCharacter.bOnInteraction` _asbp_third_person_character)
      (if (`self.bDialogueStarted`)
        (if (< _dialogueindex (- _returnvalue 1))
          (bind _result (`/Engine/EditorBlueprintResources/StandardMacros.IncrementInt` _dialogueindex)
            (:`  `
              (set `self.ActualTextDialogue` (`|GetArrayItem` _dialoguetext _result))
              (if (== (+ _result 1) _returnvalue)
                (bind _sceneloaderref (`self.SceneLoaderRef`)
                  (:`then`
                    (`/Game/Hibiki/01_Blueprints/SceneManagement/BP_SceneLoader.LoadScene` _sceneloaderref)
                    (`/Engine/EditorBlueprintResources/StandardMacros.IsValid` _doortounlock
                      (:`Is Valid`
                        (`/Game/Hibiki/01_Blueprints/BP_Door.SetDoorUnlockVisual` _doortounlock)
                        (bind _asbp_third_person_character_2 (cast `/Game/Hibiki/01_Blueprints/Characters/BP_PlayerCharacter` (`GameplayStatics.GetPlayerCharacter` 0)))
                        (`GameplayStatics.ApplyDamage` _asbp_third_person_character_2 10.0))))
                  (:`else`)))))
          (else
            (`/Engine/EditorBlueprintResources/StandardMacros.IsValid` _ui_maindialogue
              (:`Is Valid`
                (`Widget.RemoveFromParent` _ui_maindialogue)
                (`self.EnableInput` (`GameplayStatics.GetPlayerCharacter` 0) (`GameplayStatics.GetPlayerController` 0))))))
        (else
          (`/Engine/EditorBlueprintResources/StandardMacros.DoOnce` false
            (:`Completed`
              (`self.DisableInput` (`GameplayStatics.GetPlayerCharacter` 0) (`GameplayStatics.GetPlayerController` 0))
              (bind _returnvalue_2 (`|CreateWidget` "/Game/Hibiki/01_Blueprints/UI/WB_MainDialogue.WB_MainDialogue_C" (`GameplayStatics.GetPlayerController` 0)))
              (bind _output_get (set `self.UI_MainDialogue` _returnvalue_2))
              (`UserWidget.AddToViewport` _output_get 0)
              (set `/Game/Hibiki/01_Blueprints/UI/WB_MainDialogue.BP_PNJ` self (`self.UI_MainDialogue`))
              (bind _result_2 (`/Engine/EditorBlueprintResources/StandardMacros.IncrementInt` (`self.DialogueIndex`))
                (:`  `
                  (set `self.ActualTextDialogue` (`|GetArrayItem` (`self.DialogueText`) _result_2))
                  (set `self.bDialogueStarted` true))))))))))

(fn `UserConstructionScript`)