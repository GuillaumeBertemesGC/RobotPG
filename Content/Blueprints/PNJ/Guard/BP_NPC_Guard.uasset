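; BP_NPC_Guard is a guard NPC that can unlock an assigned door.
; The construction script writes CharacterName to a name text component, which SetInteractibleState shows or hides.
; ConversationClosed notifies the interaction instigator, and Unlock_Guarded_Door calls UnlockDoor on DoorToUnlock when that reference is valid.
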(event `/Game/Blueprints/BP_Interactiblee.SetInteractibleState`
  (params (`bCanSowInteract?` :type Boolean))
  (if `bCanSowInteract?`
    (`SceneComponent.SetVisibility` (`self.Txt_CharacterName`) true false)
    (else
      (`SceneComponent.SetVisibility` (`self.Txt_CharacterName`) false false))))

(event `/Game/Blueprints/BP_Interactiblee.ConversationClosed`
  (message `/Game/Blueprints/BP_Interactiblee.ConversationClosed` (`self.InteractInstigator`)))

(event `Unlock_Guarded_Door`
  (bind _doortounlock (`self.DoorToUnlock`))
  (`/Engine/EditorBlueprintResources/StandardMacros.IsValid` _doortounlock
    (:`Is Valid`
      (`/Game/SciFi_BioLaboratory/Blueprints/BP_Door.UnlockDoor` _doortounlock))))

(fn `UserConstructionScript`
  (`TextRenderComponent.K2_SetText` (`self.Txt_CharacterName`) (`self.CharacterName`)))