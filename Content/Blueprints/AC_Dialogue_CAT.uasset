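; AC_Dialogue_CAT is a dialogue component that scripts the French conversation with the character C.A.T.
; It overrides Dialogue, calls the parent, then chains AddDialogue nodes under tree index 0, advancing on each Pass Through state.
; Meowing back closes the conversation with false, while barking draws a complaint and a pointer to its friend Mouse before closing with true.
; Both endings clear dialogue progress first.
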(fn `Dialogue`
  (`parent.Dialogue`)
  (switch `int` (`self.DialogueTreeIndex`)
    (:`0`
      (bind (_state _optionindex) (`self.AddDialogue` "C.A.T" "Bip bip, miaou!" (`|MakeArray` "Miaou!" "Ouaf!." :!type "Text")))
      (switch `/Game/Blueprints/Enum_DialogueState` _state
        (:`NewEnumerator0`
          (switch `int` _optionindex
            (:`0`
              (`self.ClearDialogueProgress`)
              (`self.CloseConversation` false))
            (:`1`
              (bind _state_2 (`self.AddDialogue` "C.A.T" "Hey là! \nNe te moque pas de moi non plus..." (`|MakeArray` "Désolé." :!type "Text")))
              (switch `/Game/Blueprints/Enum_DialogueState` _state_2
                (:`NewEnumerator0`
                  (bind _state_3 (`self.AddDialogue` "C.A.T" "Si tu veux embêter quelqu'un, \nva plutôt voir mon copain Mouse! \nBip bip, miaou!" (`|MakeArray` "Avec plaisir!." :!type "Text")))
                  (switch `/Game/Blueprints/Enum_DialogueState` _state_3
                    (:`NewEnumerator0`
                      (`self.ClearDialogueProgress`)
                      (`self.CloseConversation` true))))))))))))