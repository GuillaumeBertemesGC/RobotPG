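; Game-instance-style context that carries combat, save progress and audio state across levels.
; Combat callers store pending NPC, door and checkpoint data; on battle exit, a win saves them and flags an NPC spawn, and either result reopens L_Level_1.
; Save helpers sync BP_SaveGame with cached progress.
; Music crossfades through level-persistent 2D sounds with one-step history, ignoring RequestMusic's FadeTime, while saved settings drive sound-mix volumes.
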(event `self.ReceiveInit`
  (add `self.ExitBattle` (delegate `OnBattleExit`)))

(event `OnBattleExit`
  (`KismetSystemLibrary.PrintString` (`KismetTextLibrary.Conv_TextToString` (`|FormatText` "Battle Exit with {a} result" (`self.Succedeed`))) true true (struct :`R` 1.0 :`G` 0.713203 :`A` 1.0) 10.0)
  (if (`self.Succedeed`)
    (`self.OnCombatWin`)
    (else
      (`self.OnCombatLoss`))))

(fn `DoesSaveGameExist_Hibiki`
  (returns (ReturnValue :type Boolean))
  (bind _returnvalue (`GameplayStatics.DoesSaveGameExist` (`self.SaveSlotName`)))
  (return _returnvalue))

(fn `InitOrLoadSave`
  (bind _returnvalue (`self.DoesSaveGameExist_Hibiki`))
  (if _returnvalue
    (bind _returnvalue_2 (`GameplayStatics.LoadGameFromSlot` (`self.SaveSlotName`)))
    (bind _asbp_save_game (cast `/Game/Hibiki/01_Blueprints/SceneManagement/Save/BP_SaveGame` _returnvalue_2))
    (bind _output_get (set `self.CurrentSaveGame` _asbp_save_game))
    (`self.SetContextFromSave` _output_get)
    (else
      (bind _returnvalue_3 (`GameplayStatics.CreateSaveGameObject` "/Game/Hibiki/01_Blueprints/SceneManagement/Save/BP_SaveGame.BP_SaveGame_C"))
      (bind _output_get_2 (set `self.CurrentSaveGame` _returnvalue_3))
      (`GameplayStatics.SaveGameToSlot` _output_get_2 (`self.SaveSlotName`))
      (`self.SetContextFromSave` _output_get_2))))

(fn `OnCombatLoss`
  (set `self.bShouldSpawnOnNPC?` false)
  (`GameplayStatics.OpenLevelBySoftObjectPtr` "/Game/Hibiki/02_Maps/L_Level_1.L_Level_1"))

(fn `OnCombatWin`
  (bind _currentsavegame (`self.CurrentSaveGame`))
  (`self.CurrentSaveGame`
    (:`then`
      _)
    (:`else`
      (bind _returnvalue (`GameplayStatics.CreateSaveGameObject` "/Game/Hibiki/01_Blueprints/SceneManagement/Save/BP_SaveGame.BP_SaveGame_C"))
      (set `self.CurrentSaveGame` _returnvalue)))
  (`KismetArrayLibrary.Array_AddUnique` (`/Game/Hibiki/01_Blueprints/SceneManagement/Save/BP_SaveGame.DefeatedNPCIDs` _currentsavegame) (`self.PendingNPCID`))
  (`KismetArrayLibrary.Array_AddUnique` (`/Game/Hibiki/01_Blueprints/SceneManagement/Save/BP_SaveGame.UnlockedDoorIDs` _currentsavegame) (`self.PendingLinkedDoorID`))
  (set `/Game/Hibiki/01_Blueprints/SceneManagement/Save/BP_SaveGame.CurrentCheckpointId` (`self.CurrentCheckpointId`) _currentsavegame)
  (set `/Game/Hibiki/01_Blueprints/SceneManagement/Save/BP_SaveGame.PlayerStats` (`self.PlayerStats`) _currentsavegame)
  (set `self.bShouldSpawnOnNPC?` true)
  (`GameplayStatics.SaveGameToSlot` (`self.CurrentSaveGame`) (`self.SaveSlotName`))
  (`GameplayStatics.OpenLevelBySoftObjectPtr` "/Game/Hibiki/02_Maps/L_Level_1.L_Level_1"))

(fn `OverwriteSave`
  (bind _returnvalue (`GameplayStatics.CreateSaveGameObject` "/Game/Hibiki/01_Blueprints/SceneManagement/Save/BP_SaveGame.BP_SaveGame_C"))
  (bind _output_get (set `self.CurrentSaveGame` _returnvalue))
  (`GameplayStatics.SaveGameToSlot` _output_get (`self.SaveSlotName`))
  (`self.SetContextFromSave` _output_get))

(fn `PlayExplorationMusic`
  (params (FadeTime :type "Float (double-precision)" :default 1.5))
  (`self.RequestMusic` (`self.ExploMusic`) FadeTime))

(fn `PlayMenuMusic`
  (params (FadeTime :type "Float (double-precision)" :default 1.0))
  (`self.RequestMusic` (`self.MenuMusic`) FadeTime))

(fn `RequestMusic`
  (params (NewMusic :type "SoundBase Object Reference") (FadeTime :type "Float (double-precision)") (SaveAsPrevious :type Boolean))
  (locals (OldMusicComponent :type "AudioComponent Object Reference"))
  (`/Engine/EditorBlueprintResources/StandardMacros.IsValid` NewMusic
    (:`Is Valid`
      (if (!= (`self.CurrentMusic`) NewMusic)
        (if (`local.SaveAsPrevious`)
          (set `self.PreviousMusic` (`self.CurrentMusic`)))
        (bind _output_get (set `local.OldMusicComponent` (`self.CurrentMusicComponent`)))
        (`/Engine/EditorBlueprintResources/StandardMacros.IsValid` _output_get
          (:`Is Valid`
            (`AudioComponent.FadeOut` _output_get (`self.MusicFadeDuration`) 0.0 "Linear"))
          (:`Is Not Valid`
            _))
        (bind _returnvalue (`GameplayStatics.CreateSound2D` (`local.NewMusic`) 1.0 1.0 0.0 null true))
        (bind _output_get_2 (set `self.CurrentMusicComponent` _returnvalue))
        (set `self.CurrentMusic` (`local.NewMusic`))
        (`AudioComponent.FadeIn` _output_get_2 (`self.MusicFadeDuration`) 1.0 0.0 "Linear")
        (else
          (return))))
    (:`Is Not Valid`
      (return))))

(fn `ReturnToPreviousMusic`
  (params (FadeTime :type "Float (double-precision)"))
  (bind _previousmusic (`self.PreviousMusic`)
    (:`then`
      (`self.RequestMusic` _previousmusic FadeTime)
      (set `self.PreviousMusic` null))
    (:`else`)))

(fn `SaveAllDatas`
  (bind _currentsavegame (`self.CurrentSaveGame`)
    (:`then`
      (set `/Game/Hibiki/01_Blueprints/SceneManagement/Save/BP_SaveGame.DefeatedNPCIDs` (`self.DefeatedNPCIDs`) _currentsavegame)
      (set `/Game/Hibiki/01_Blueprints/SceneManagement/Save/BP_SaveGame.UnlockedDoorIDs` (`self.UnlockedDoorIDs`) _currentsavegame)
      (set `/Game/Hibiki/01_Blueprints/SceneManagement/Save/BP_SaveGame.CurrentCheckpointId` (`self.CurrentCheckpointId`) _currentsavegame)
      (set `/Game/Hibiki/01_Blueprints/SceneManagement/Save/BP_SaveGame.PlayerStats` (`self.PlayerStats`) _currentsavegame))
    (:`else`
      (bind _returnvalue (`GameplayStatics.CreateSaveGameObject` "/Game/Hibiki/01_Blueprints/SceneManagement/Save/BP_SaveGame.BP_SaveGame_C"))
      (set `self.CurrentSaveGame` _returnvalue)))
  (`GameplayStatics.SaveGameToSlot` (`self.CurrentSaveGame`) (`self.SaveSlotName`)))

(fn `SaveCheckpointId`
  (params (CurrentCheckpointId :type Name))
  (bind _saveslotname (`self.SaveSlotName`))
  (set `self.CurrentCheckpointId` CurrentCheckpointId)
  (bind _returnvalue (`self.DoesSaveGameExist_Hibiki`))
  (if _returnvalue
    (bind _returnvalue_2 (`GameplayStatics.LoadGameFromSlot` (`self.SaveSlotName`)))
    (bind _asbp_save_game (cast `/Game/Hibiki/01_Blueprints/SceneManagement/Save/BP_SaveGame` _returnvalue_2))
    (set `/Game/Hibiki/01_Blueprints/SceneManagement/Save/BP_SaveGame.CurrentCheckpointId` (`self.CurrentCheckpointId`) _asbp_save_game)
    (`GameplayStatics.SaveGameToSlot` _asbp_save_game _saveslotname)
    (else
      (bind _returnvalue_3 (`GameplayStatics.CreateSaveGameObject` "/Game/Hibiki/01_Blueprints/SceneManagement/Save/BP_SaveGame.BP_SaveGame_C"))
      (set `/Game/Hibiki/01_Blueprints/SceneManagement/Save/BP_SaveGame.CurrentCheckpointId` (`self.CurrentCheckpointId`) _returnvalue_3)
      (`GameplayStatics.SaveGameToSlot` _returnvalue_3 _saveslotname))))

(fn `SetCombatContext`
  (params (CombatConfig :type "/Game/Scripts/BP/Battle/Data/BP_DA_CombatConfig Object Reference") (NPCID :type Name) (DoorID :type Name) (SpawnTransform :type "Transform Structure") (CurrentCheckpointId :type Name))
  (set `self.CurrentCombatData` CombatConfig)
  (set `self.PendingNPCID` NPCID)
  (set `self.PendingLinkedDoorID` DoorID)
  (set `self.PendingNPCCheckpointTransform` SpawnTransform)
  (set `self.CurrentCheckpointId` CurrentCheckpointId))

(fn `SetContextFromSave`
  (params (Savegame :type "/Game/Hibiki/01_Blueprints/SceneManagement/Save/BP_SaveGame Object Reference"))
  (set `self.DefeatedNPCIDs` (`/Game/Hibiki/01_Blueprints/SceneManagement/Save/BP_SaveGame.DefeatedNPCIDs` Savegame))
  (set `self.UnlockedDoorIDs` (`/Game/Hibiki/01_Blueprints/SceneManagement/Save/BP_SaveGame.UnlockedDoorIDs` Savegame))
  (set `self.CurrentCheckpointId` (`/Game/Hibiki/01_Blueprints/SceneManagement/Save/BP_SaveGame.CurrentCheckpointId` Savegame))
  (set `self.PlayerStats` (`/Game/Hibiki/01_Blueprints/SceneManagement/Save/BP_SaveGame.PlayerStats` Savegame)))

(fn `SetSoundMixVolumes`
  (bind _nameslot_ (`/Game/MGS_vs_DownGrade/Blueprint/BP_SettingsLibrary.SettingsSlotNameSaveGame`))
  (bind _returnvalue (`GameplayStatics.DoesSaveGameExist` _nameslot_))
  (if _returnvalue
    (bind _returnvalue_2 (`GameplayStatics.LoadGameFromSlot` _nameslot_))
    (bind _asbp_save_graphics (cast `/Game/MGS_vs_DownGrade/Blueprint/BP_SaveGraphics` _returnvalue_2)
      (:`then`
        (bind _output_get (set `self.SaveSettings` _asbp_save_graphics))
        (`GameplayStatics.SetSoundMixClassOverride` "/Game/Hibiki/07_Sfx/AudioManager/HBK_SoundMix.HBK_SoundMix" "/Game/Hibiki/07_Sfx/AudioManager/HBK_SC_Master.HBK_SC_Master" (`/Game/MGS_vs_DownGrade/Blueprint/BP_SaveGraphics.MasterVolume` _output_get) 1.0 0.0)
        (`GameplayStatics.PushSoundMixModifier` "/Game/Hibiki/07_Sfx/AudioManager/HBK_SoundMix.HBK_SoundMix")
        (`GameplayStatics.SetSoundMixClassOverride` "/Game/Hibiki/07_Sfx/AudioManager/HBK_SoundMix.HBK_SoundMix" "/Game/Hibiki/07_Sfx/AudioManager/HBK_SC_Music.HBK_SC_Music" (`/Game/MGS_vs_DownGrade/Blueprint/BP_SaveGraphics.MusicVolume` _output_get) 1.0 0.0)
        (`GameplayStatics.PushSoundMixModifier` "/Game/Hibiki/07_Sfx/AudioManager/HBK_SoundMix.HBK_SoundMix")
        (`GameplayStatics.SetSoundMixClassOverride` "/Game/Hibiki/07_Sfx/AudioManager/HBK_SoundMix.HBK_SoundMix" "/Game/Hibiki/07_Sfx/AudioManager/HBK_SC_Sfx.HBK_SC_Sfx" (`/Game/MGS_vs_DownGrade/Blueprint/BP_SaveGraphics.SfxVolume` _output_get) 1.0 0.0)
        (`GameplayStatics.PushSoundMixModifier` "/Game/Hibiki/07_Sfx/AudioManager/HBK_SoundMix.HBK_SoundMix"))
      (:`CastFailed`
        (`GameplayStatics.SetSoundMixClassOverride` "/Game/Hibiki/07_Sfx/AudioManager/HBK_SoundMix.HBK_SoundMix" "/Game/Hibiki/07_Sfx/AudioManager/HBK_SC_Master.HBK_SC_Master" 1.0 1.0 0.0 :!label _label)
        (`GameplayStatics.PushSoundMixModifier` "/Game/Hibiki/07_Sfx/AudioManager/HBK_SoundMix.HBK_SoundMix")
        (`GameplayStatics.SetSoundMixClassOverride` "/Game/Hibiki/07_Sfx/AudioManager/HBK_SoundMix.HBK_SoundMix" "/Game/Hibiki/07_Sfx/AudioManager/HBK_SC_Music.HBK_SC_Music" 1.0 1.0 0.0)
        (`GameplayStatics.PushSoundMixModifier` "/Game/Hibiki/07_Sfx/AudioManager/HBK_SoundMix.HBK_SoundMix")
        (`GameplayStatics.SetSoundMixClassOverride` "/Game/Hibiki/07_Sfx/AudioManager/HBK_SoundMix.HBK_SoundMix" "/Game/Hibiki/07_Sfx/AudioManager/HBK_SC_Sfx.HBK_SC_Sfx" 1.0 1.0 0.0)
        (`GameplayStatics.PushSoundMixModifier` "/Game/Hibiki/07_Sfx/AudioManager/HBK_SoundMix.HBK_SoundMix")))
    (else
      (goto _label))))

(fn `StopCombatMusic`
  (params (FadeTime :type "Float (double-precision)" :default 1.5))
  (`self.ReturnToPreviousMusic` FadeTime))

(fn `StopMusic`
  (params (FadeTime :type "Float (double-precision)"))
  (bind _currentmusiccomponent (`self.CurrentMusicComponent`)
    (:`then`
      (`AudioComponent.FadeOut` _currentmusiccomponent FadeTime 0.0 "Linear"))
    (:`else`
      _))
  (set `self.CurrentMusic` null)
  (set `self.CurrentMusicComponent` null))