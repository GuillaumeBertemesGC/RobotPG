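; Dialogue component for the Mouse NPC, a short French conversation in which the mouse asks the player for cheese.
; Overrides Dialogue, calls the parent, then branches on tree index and chosen option through nested AddDialogue calls, some with audio or animation.
; Claiming to have cheese leads to a confession and a peaceful close.
; Refusing closes the conversation, stores combat data in the Context game instance and opens the battle level.
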(fn `Dialogue`
  (`parent.Dialogue`)
  (switch `int` (`self.DialogueTreeIndex`)
    (:`0`
      (bind (_state _optionindex) (`self.AddDialogue` "Mouse" "Salut, t'aurais pas du fromage?" (`|MakeArray` "Oui, bien sûr!" "Non." :!type "Text")))
      (switch `/Game/Blueprints/Enum_DialogueState` _state
        (:`NewEnumerator0`
          (switch `int` _optionindex
            (:`0`
              (bind (_state_2 _optionindex_2) (`self.AddDialogue` "Mouse" "Incroyable, il en existe encore? \nJe pensais qu'il avais tous disparus ! ^^" (`|MakeArray` "En faite, je n'en ai pas." :!type "Text") "/Game/StarterContent/Audio/Explosion01.Explosion01" null "NewEnumerator1"))
              (switch `/Game/Blueprints/Enum_DialogueState` _state_2
                (:`NewEnumerator0`
                  (switch `int` _optionindex_2
                    (:`0`
                      (bind _state_3 (`self.AddDialogue` "Mouse" "Ha...." (`|MakeArray` "Bonne journée!" :!type "Text") null null "NewEnumerator2"))
                      (switch `/Game/Blueprints/Enum_DialogueState` _state_3
                        (:`NewEnumerator0`
                          (`self.ClearDialogueProgress`)
                          (`self.CloseConversation` false))))))))
            (:`1`
              (bind _state_4 (`self.AddDialogue` "Mouse" "Dommage T-T" (`|MakeArray` "Au revoir!" :!type "Text")))
              (switch `/Game/Blueprints/Enum_DialogueState` _state_4
                (:`NewEnumerator0`
                  (`self.ClearDialogueProgress`)
                  (`self.CloseConversation` false)
                  (bind _ascontext (cast `/Game/Hibiki/01_Blueprints/SceneManagement/Context` (`GameplayStatics.GetGameInstance`)))
                  (set `/Game/Hibiki/01_Blueprints/SceneManagement/Context.CurrentCombatData` (`self.Current Combat Data`) _ascontext)
                  (`GameplayStatics.OpenLevelBySoftObjectPtr` "/Game/Hibiki/02_Maps/L_Battle.L_Battle"))))))))))