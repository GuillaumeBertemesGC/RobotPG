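; Dialogue component for the second tutorial guard, Guard_Tuto_2, offering the player a choice in French between staying calm and fighting.
; It overrides Dialogue, calls the parent, then builds tree index 0 from nested AddDialogue calls, advancing on Pass Through and branching on the chosen option.
; Staying calm clears progress and closes the conversation with false; fighting goes through two confirmation lines, then clears progress and closes with true.
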(fn `Dialogue`
  (`parent.Dialogue`)
  (switch `int` (`self.DialogueTreeIndex`)
    (:`0`
      (bind (_state _optionindex) (`self.AddDialogue` "Guard_Tuto_2" "Bonjour, tu veux quoi ?" (`|MakeArray` "Restons calme." "Je veux combattre." :!type "Text")))
      (switch `/Game/Blueprints/Enum_DialogueState` _state
        (:`NewEnumerator0`
          (switch `int` _optionindex
            (:`0`
              (`self.ClearDialogueProgress`)
              (`self.CloseConversation` false))
            (:`1`
              (bind _state_2 (`self.AddDialogue` "Guard_Tuto_2" "Tu es sûr ?" (`|MakeArray` "Oui." :!type "Text")))
              (switch `/Game/Blueprints/Enum_DialogueState` _state_2
                (:`NewEnumerator0`
                  (bind _state_3 (`self.AddDialogue` "Guard_Tuto_2" "C'est l'heur du dudududududduduel" (`|MakeArray` "Yu gi oh !!!" :!type "Text")))
                  (switch `/Game/Blueprints/Enum_DialogueState` _state_3
                    (:`NewEnumerator0`
                      (`self.ClearDialogueProgress`)
                      (`self.CloseConversation` true))))))))))))