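; BP_Door is an automatic double sliding door that opens when BP_ThirdPersonCharacter enters its Box trigger and closes when it leaves.
; BeginPlay caches the closed relative locations of both door meshes.
; Overlap begin and end play and reverse one Timeline, whose track lerps the meshes apart along relative X by SideDistance.
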(event `self.ReceiveBeginPlay`
  (set `self.LeftDoorClosePos` (`SceneComponent.RelativeLocation` (`self.SM_Door_Left`)))
  (set `self.RightDoorClosePos` (`SceneComponent.RelativeLocation` (`self.SM_Door_Right`))))

(event `self.Box.OnComponentBeginOverlap`
  (params (OverlappedComponent :type "PrimitiveComponent Object Reference") (OtherActor :type "Actor Object Reference") (OtherComp :type "PrimitiveComponent Object Reference") (OtherBodyIndex :type Integer) (bFromSweep :type Boolean) (SweepResult :type "HitResult Structure (by ref)"))
  (bind _leftdoorclosepos (`self.LeftDoorClosePos`))
  (bind _rightdoorclosepos (`self.RightDoorClosePos`))
  (bind _returnvalue (`KismetMathLibrary.MakeVector` (`self.SideDistance`)))
  (cast `/Game/ThirdPerson/Blueprints/BP_ThirdPersonCharacter` OtherActor)
  (bind (_direction _newtrack_0) (`Timeline|Timeline` :!label _label)
    (:`Update`
      (`SceneComponent.K2_SetRelativeLocation` (`self.SM_Door_Left`) (`KismetMathLibrary.VLerp` _leftdoorclosepos (- _leftdoorclosepos _returnvalue) _newtrack_0) false false)
      (`SceneComponent.K2_SetRelativeLocation` (`self.SM_Door_Right`) (`KismetMathLibrary.VLerp` _rightdoorclosepos (+ _rightdoorclosepos _returnvalue) _newtrack_0) false false))))

(event `self.Box.OnComponentEndOverlap`
  (params (OverlappedComponent :type "PrimitiveComponent Object Reference") (OtherActor :type "Actor Object Reference") (OtherComp :type "PrimitiveComponent Object Reference") (OtherBodyIndex :type Integer))
  (cast `/Game/ThirdPerson/Blueprints/BP_ThirdPersonCharacter` OtherActor)
  (goto _label :!via `Reverse`))

(fn `UserConstructionScript`)